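; Spline-driven vine foliage actor that builds a chain of spline meshes along an editable Spline component.
; The construction script adds one X-forward spline mesh per segment, matching local positions and tangents of neighboring points.
; Separate branches handle first, middle and last segments with identical logic, each through its own component node.
; The event graph holds only disabled stub events, so there is no runtime logic.
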(event EventBeginPlay)

(event Collision|EventActorBeginOverlap
  (params (OtherActor :type Actor%20Object%20Reference)))

(event EventTick
  (params (DeltaSeconds :type Float%20%28single-precision%29)))

(fn ConstructionScript
  (bind _spline (Variables|Default|GetSpline))
  (bind _spline_2 (Variables|Default|GetSpline))
  (bind _spline_3 (Variables|Default|GetSpline))
  (bind _spline_4 (Variables|Default|GetSpline))
  (bind _spline_5 (Variables|Default|GetSpline))
  (bind _spline_6 (Variables|Default|GetSpline))
  (bind _spline_7 (Variables|Default|GetSpline))
  (bind _returnvalue (Spline|GetNumberOfSplinePoints _spline))
  (bind _returnvalue_2 (- _returnvalue 2))
  (for _index (range 0 _returnvalue_2)
    (if (== _index 0)
      ;[1 1 1] First mesh
      (bind _returnvalue_3 (AddComponent|AddSplineMeshComponent false))
      (SplineMesh|SetForwardAxis _returnvalue_3 "X" true)
      (SplineMesh|SetStartandEnd _returnvalue_3 (Spline|GetLocationatSplinePoint _spline_6 _index "Local") (Spline|GetTangentatSplinePoint _spline_6 _index "Local") (Spline|GetLocationatSplinePoint _spline_7 (+ _index 1) "Local") (Spline|GetTangentatSplinePoint _spline_7 (+ _index 1) "Local") true :!class /Script/Engine.SplineMeshComponent)
      (elif (== _index _returnvalue_2)
        ;[1 1 1] Last Mesh
        (bind _returnvalue_4 (AddComponent|AddSplineMeshComponent false))
        (SplineMesh|SetForwardAxis _returnvalue_4 "X" true)
        (SplineMesh|SetStartandEnd _returnvalue_4 (Spline|GetLocationatSplinePoint _spline_2 _index "Local") (Spline|GetTangentatSplinePoint _spline_2 _index "Local") (Spline|GetLocationatSplinePoint _spline_3 (+ _index 1) "Local") (Spline|GetTangentatSplinePoint _spline_3 (+ _index 1) "Local") true :!class /Script/Engine.SplineMeshComponent)
        (else
          ;[1 1 1] Between mesh
          (bind _returnvalue_5 (AddComponent|AddSplineMeshComponent false))
          (SplineMesh|SetForwardAxis _returnvalue_5 "X" true)
          (SplineMesh|SetStartandEnd _returnvalue_5 (Spline|GetLocationatSplinePoint _spline_4 _index "Local") (Spline|GetTangentatSplinePoint _spline_4 _index "Local") (Spline|GetLocationatSplinePoint _spline_5 (+ _index 1) "Local") (Spline|GetTangentatSplinePoint _spline_5 (+ _index 1) "Local") true :!class /Script/Engine.SplineMeshComponent))))))