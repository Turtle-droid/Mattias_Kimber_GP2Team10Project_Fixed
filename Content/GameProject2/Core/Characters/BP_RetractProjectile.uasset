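; BP_RetractProjectile is a homing projectile that travels toward a Target actor and disappears when it reaches the player.
; On BeginPlay it rotates to face the Target from its Sphere location and sets the Target's root as the ProjectileMovement homing component.
; When the Sphere begins overlapping a BP_PlayerPawn, the projectile destroys itself, with no other effect applied to the pawn.
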(event OnComponentBeginOverlap(Sphere)
  (params (OverlappedComponent :type Primitive%20Component%20Object%20Reference) (OtherActor :type Actor%20Object%20Reference) (OtherComp :type Primitive%20Component%20Object%20Reference) (OtherBodyIndex :type Integer) (bFromSweep :type Boolean) (SweepResult :type Hit%20Result%20Structure%20%28by%20ref%29))
  (Utilities|Casting|CastToBP_PlayerPawn OtherActor)
  (Actor|DestroyActor))

(event EventBeginPlay
  (Transformation|SetActorRotation (Math|Rotator|FindLookatRotation (Transformation|GetWorldLocation (Variables|Default|GetSphere self)) (Transformation|GetActorLocation (Variables|Default|GetTarget))))
  (Variables|/Script/Engine.ProjectileMovementComponent|SetHomingTargetComponent (Variables|Default|GetProjectileMovement) (Variables|/Script/Engine.Actor|GetRootComponent (Variables|Default|GetTarget))))

(fn ConstructionScript)