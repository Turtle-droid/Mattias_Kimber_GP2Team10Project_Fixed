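; Rope endpoint attached to an actor, paired with another rope point to drag objects together.
; While pulling, Tick pushes its movable mesh toward the partner beyond a minimum distance, or flags both points for player-pawn cleanup if its actor is gone.
; Stiffen swaps pulling for a spawned physics constraint between both meshes and changes the cable material; release reverses this.
; Toggling pulling on enables breakable physics, and a timer briefly flashes the sphere red.
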(event Custom|PullingTowards
  (params (OtherHit :type BP%20Rope%20Points%20Object%20Reference))
  ;[1 1 1] Pulling Towards other point
  (Variables|Default|SetOtherHit OtherHit))

(event Custom|TogglePulling
  ;[1 1 1] Toggle
  (if (Variables|Default|GetIsPulling)
    (Variables|Default|SetIsPulling false)
    (else
      (Variables|Default|SetIsPulling true)
      (bind _asthe_breakabled (Utilities|Casting|CastToThe_Breakabled (Variables|Default|GetOtherActor)))
      (Physics|SetSimulatePhysics (Variables|/Game/GameProject2/Placeables/Moveables/Breakable_Blocks/The_Breakabled.The_Breakabled_C|GetStaticMesh _asthe_breakabled) true))))

(event Custom|ToggleRed
  ;[1 1 1] Pulling Towards other point
  (Variables|Default|SetRedTimer 0.1)
  (Rendering|Material|SetMaterial (Variables|Default|GetSphere) 0 "/Game/GameProject2/Core/Characters/M_RopeRed.M_RopeRed"))

(event Custom|Stiffen
  (bind _otherhit (Variables|Default|GetOtherHit))
  ;[1 1 1] Stiffen Rope
  (Variables|Default|GetOtherHit
    (:then
      (bind _returnvalue (Game|SpawnActorfromClass "/Script/Engine.PhysicsConstraintActor" (Math|Conversions|ToTransform(Vector) (Transformation|GetWorldLocation (Variables|Default|GetSphere self))) "Undefined" 0 0))
      (bind _output_get (Variables|Default|SetPConstraint _returnvalue))
      (Variables|BP_RopePoints_C|GetPConstraint _otherhit
        (:then
          _)
        (:else
          (Variables|BP_RopePoints_C|SetPConstraint _otherhit _output_get)))
      (Rendering|Material|SetMaterial (Variables|/Script/CableComponent.CableActor|GetCableComponent (Variables|Default|GetCable)) 0 "/Game/GameProject2/Effects/FXAssets/MI_RopeShader.MI_RopeShader")
      (Class|PhysicsConstraintComponent|SetConstrainedComponents (Variables|/Script/Engine.PhysicsConstraintActor|GetConstraintComp _returnvalue) (Actor|GetComponentbyClass (Variables|Default|GetOtherActor) "/Script/Engine.StaticMeshComponent") "None" (Actor|GetComponentbyClass (Variables|BP_RopePoints_C|GetOtherActor (Variables|Default|GetOtherHit)) "/Script/Engine.StaticMeshComponent") "None")
      (Development|PrintString "ATTACHED")
      (Variables|Default|SetIsPulling false))
    (:else)))

(event Custom|Release%20Stiffen
  ;[1 1 1] Release Stiffen
  (bind _pconstraint (Variables|Default|GetPConstraint)
    (:then
      (Actor|DestroyActor _pconstraint))
    (:else
      _))
  (bind _pconstraint_2 (Variables|BP_RopePoints_C|GetPConstraint (Variables|Default|GetOtherHit))
    (:then
      (Actor|DestroyActor _pconstraint_2))
    (:else
      _))
  (Rendering|Material|SetMaterial (Variables|/Script/CableComponent.CableActor|GetCableComponent (Variables|Default|GetCable)) 0 "/Game/GameProject2/Effects/FXAssets/M_RopeShader.M_RopeShader")
  (Variables|Default|SetIsPulling true))

(event EventTick
  (params (DeltaSeconds :type Float%20%28single-precision%29))
  (bind _otheractor (Variables|Default|GetOtherActor))
  (bind _returnvalue (Actor|GetComponentbyClass _otheractor "/Script/Engine.StaticMeshComponent"))
  ;[1 1 1] Pulling Towards other point
  (Utilities|FlowControl|Sequence
    (:then_0
      (bind _output_get (Variables|Default|SetRedTimer (- (Variables|Default|GetRedTimer) DeltaSeconds)))
      (if (< _output_get 0.0)
        (Rendering|Material|SetMaterial (Variables|Default|GetSphere) 0 "/Game/GameProject2/MaterialLibrary/M_Ammo_Seethrough.M_Ammo_Seethrough")))
    (:then_1
      (if (Variables|Default|GetIsPulling)
        (Utilities|FlowControl|Sequence
          (:then_0
            (Variables|Default|GetOtherActor
              (:then
                (if (Utilities|Enum|Equal(Enum) (Variables|/Script/Engine.SceneComponent|GetMobility _returnvalue) "Movable")
                  (if (> (Math|Vector|VectorLength (- (Transformation|GetWorldLocation (Variables|BP_RopePoints_C|GetSphere (Variables|Default|GetOtherHit))) (Transformation|GetWorldLocation (Variables|Default|GetDefaultSceneRoot)))) 4e+02)
                    (Class|PrimitiveComponent|AddForceatLocation _returnvalue (* (Math|Vector|Normalize (- (Transformation|GetWorldLocation (Variables|BP_RopePoints_C|GetDefaultSceneRoot (Variables|Default|GetOtherHit))) (Transformation|GetWorldLocation (Variables|Default|GetDefaultSceneRoot self)))) (+ (Variables|Default|GetForce) (Variables|Default|GetCharge))) (Transformation|GetWorldLocation (Variables|Default|GetDefaultSceneRoot self)) "None"))))
              (:else
                (Variables|Default|SetMarked true)
                (Variables|BP_RopePoints_C|SetMarked (Variables|Default|GetOtherHit) true)
                (Default|RemoveMarkedThings (.AsBP%20Player%20Pawn (Utilities|Casting|CastToBP_PlayerPawn (Pawn|GetControlledPawn (Game|GetPlayerController 0)))))))))))))

(fn ConstructionScript)