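; BP_PlayerHealthComponent is a health component that tracks the player's health and signals death.
; ApplyDamage subtracts damage, clamps health between zero and the maximum, then runs CheckForDeath, which calls OnDeath when health reaches zero.
; A DoOnce gate keeps death from firing repeatedly until ResetHealthComponent restores full health and reopens it for respawn.
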(event Custom|CheckForDeath
  ;[1 1 1] Check for death
  (if (== (Variables|Default|GetPlayerHealth) 0.0)
    (Utilities|FlowControl|DoOnce false
      (:Completed
        (Default|CallOnDeath)))))

(event Custom|ResetHealthComponent
  ;[1 1 1] Check for death
  ;;[1 1 1 1 8] reset it so that it can trigger again (get health back when you respawn)
  (Variables|Default|SetPlayerHealth (Variables|Default|GetPlayerHealthMax))
  (Utilities|FlowControl|DoOnce false) ; enters at Reset
)

(event Custom|Apply%20Damage
  (params (Damage :type Float%20%28single-precision%29))
  ;[1 1 1] Taking Damage
  (Variables|Default|SetPlayerHealth (Math|Float|Clamp(Float) (- (Variables|Default|GetPlayerHealth) Damage) 0.0 (Variables|Default|GetPlayerHealthMax)))
  (CallFunction|CheckforDeath))