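; BP_PlayerHarpoon is a harpoon projectile tied to the BP_PlayerPawn that owns it, which it caches on BeginPlay.
; When the harpoon head hits something, it reports the hit actor and head location to the player's HarpoonHit, then destroys itself.
; Tick counts down its Lifetime, and on expiry it spawns a BP_RetractProjectile at the head, targeting the player, before destroying itself.
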(event OnComponentHit(HarpoonHead)
  (params (HitComponent :type Primitive%20Component%20Object%20Reference) (OtherActor :type Actor%20Object%20Reference) (OtherComp :type Primitive%20Component%20Object%20Reference) (NormalImpulse :type Vector :default "0, 0, 0") (Hit :type Hit%20Result%20Structure%20%28by%20ref%29))
  (Default|HarpoonHit (Variables|Default|GetPlayer) OtherActor (Transformation|GetWorldLocation (Variables|Default|GetHarpoonHead)))
  (Actor|DestroyActor))

(event EventBeginPlay
  (Class|Actor|AddActorWorldRotation (Math|Rotator|MakeRotator 0.0 0.0 0.0))
  (bind _asbp_player_pawn (Utilities|Casting|CastToBP_PlayerPawn (Components|GetOwner)))
  (Variables|Default|SetPlayer _asbp_player_pawn))

(event Collision|EventActorBeginOverlap
  (params (OtherActor :type Actor%20Object%20Reference)))

(event EventTick
  (params (DeltaSeconds :type Float%20%28single-precision%29))
  (bind _harpoonhead (Variables|Default|GetHarpoonHead))
  (bind _returnvalue (Transformation|GetWorldTransform _harpoonhead))
  (bind _output_get (Variables|Default|SetLifetime (- (Variables|Default|GetLifetime) DeltaSeconds)))
  (if (< _output_get 0.0)
    (Game|SpawnActorfromClass "/Game/GameProject2/Core/Characters/BP_RetractProjectile.BP_RetractProjectile_C" (Math|Transform|MakeTransform (.location _returnvalue) (.rotation _returnvalue) "0.200000,0.200000,0.200000") "Undefined" 0 (Variables|Default|GetPlayer) 0)
    (Actor|DestroyActor)))

(fn ConstructionScript)