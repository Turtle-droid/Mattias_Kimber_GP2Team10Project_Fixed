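; Player pawn with a harpoon rope gun, air-dash effects, health upgrades, damage invincibility and debug teleports.
; Paired harpoon hits spawn BP_RopePoints linked by a CableActor and toggled to pull, up to RopeMax ropes.
; Tapping Remove retracts sphere-traced ropes under the camera's aim, while holding it retracts all via a mark-and-sweep pass.
; Pause and tutorial popups slow global time dilation to near zero rather than pausing the game.
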(event Custom|HarpoonHit
  (params (Actor :type Actor%20Object%20Reference) (Location :type Vector))
  ;[1 1 1] Spawning Rope Points
  (if (< (Variables|Default|GetAmountOfLines) (Variables|Default|GetRopeMax))
    (Variables|Default|GetCalbe
      (:then
        (bind _returnvalue (Game|SpawnActorfromClass "/Game/GameProject2/Core/Characters/BP_RopePoints.BP_RopePoints_C" (Math|Transform|MakeTransform Location "0, 0, 0" "1,1,1") "Undefined" 0 0 Actor (* (Variables|Default|GetChargePercent) 1e+04) 0))
        (Variables|Default|SetHit2 _returnvalue)
        (Transformation|AttachActorToActor _returnvalue Actor "None" "KeepWorld" "KeepWorld" "KeepWorld" true)
        (Variables|/Script/CableComponent.CableComponent|SetbAttachEnd (Variables|/Script/CableComponent.CableActor|GetCableComponent (Variables|Default|GetCalbe)) true)
        (Class|CableComponent|SetAttachEndto (Variables|/Script/CableComponent.CableActor|GetCableComponent (Variables|Default|GetCalbe)) _returnvalue "None" "None")
        (Variables|/Game/GameProject2/Core/Characters/BP_RopePoints.BP_RopePoints_C|SetOtherHit (Variables|Default|GetHit1) (Variables|Default|GetHit2))
        (Variables|/Game/GameProject2/Core/Characters/BP_RopePoints.BP_RopePoints_C|SetOtherHit (Variables|Default|GetHit2) (Variables|Default|GetHit1))
        (Variables|/Game/GameProject2/Core/Characters/BP_RopePoints.BP_RopePoints_C|SetCable (Variables|Default|GetHit2) (Variables|Default|GetCalbe))
        (Default|TogglePulling (Variables|Default|GetHit2))
        (Variables|Default|SetCalbe 0)
        (Variables|Default|SetSecondShot false)
        (Variables|Default|SetCharge 0.0)
        (Variables|Default|SetChargePercent 0.0)
        (Math|Integer|IncrementInt (Variables|Default|GetAmountOfLines)
          (:%20%20
            (switch int (- (Variables|Default|GetAmountOfLines) 1)
              (:0
                (Rendering|SetVisibility (Variables|Default|GetStaticMesh4) false false))
              (:1
                (Rendering|SetVisibility (Variables|Default|GetStaticMesh3) false false))
              (:2
                (Rendering|SetVisibility (Variables|Default|GetStaticMesh2) false false))
              (:3
                (Rendering|SetVisibility (Variables|Default|GetStaticMesh1) false false))
              (:4
                (Rendering|SetVisibility (Variables|Default|GetStaticMesh) false false))))))
      (:else
        (bind _returnvalue_2 (Game|SpawnActorfromClass "/Game/GameProject2/Core/Characters/BP_RopePoints.BP_RopePoints_C" (Math|Transform|MakeTransform Location "0, 0, 0" "1,1,1") "Undefined" 0 0 Actor (* (Variables|Default|GetChargePercent) 1e+04) 0))
        (bind _output_get (Variables|Default|SetHit1 _returnvalue_2))
        (Transformation|AttachActorToActor _output_get Actor "None" "KeepWorld" "KeepWorld" "KeepWorld" true)
        (bind _returnvalue_3 (Game|SpawnActorfromClass "/Script/CableComponent.CableActor" (Math|Transform|MakeTransform Location "0, 0, 0" "1,1,1") "Undefined" self 0))
        (bind _output_get_2 (Variables|Default|SetCalbe _returnvalue_3))
        (Rendering|Material|SetMaterial (Variables|/Script/CableComponent.CableActor|GetCableComponent _output_get_2) 0 "/Game/GameProject2/Effects/FXAssets/M_RopeShader.M_RopeShader")
        (Variables|/Game/GameProject2/Core/Characters/BP_RopePoints.BP_RopePoints_C|SetCable (Variables|Default|GetHit1) _output_get_2)
        (Transformation|AttachActorToActor _output_get_2 (Variables|Default|GetHit1) "None" "KeepWorld" "KeepWorld" "KeepWorld" true)
        (Variables|/Script/CableComponent.CableComponent|SetbAttachEnd (Variables|/Script/CableComponent.CableActor|GetCableComponent _output_get_2) false)
        (Variables|/Script/CableComponent.CableComponent|SetCableLength (Variables|/Script/CableComponent.CableActor|GetCableComponent _output_get_2) 25.0)
        (Variables|/Script/CableComponent.CableComponent|SetEndLocation (Variables|/Script/CableComponent.CableActor|GetCableComponent _output_get_2) "0, 0, 0")))))

(event Custom|RemoveMarkedThings
  ;[1 1 1] Rope deletion
  (bind _outactors (Actor|GetAllActorsOfClass "/Game/GameProject2/Core/Characters/BP_RopePoints.BP_RopePoints_C"))
  (for _array_element _outactors
    (if (Variables|/Game/GameProject2/Core/Characters/BP_RopePoints.BP_RopePoints_C|GetMarked _array_element)
      (bind _cable (Variables|/Game/GameProject2/Core/Characters/BP_RopePoints.BP_RopePoints_C|GetCable _array_element)
        (:then
          (Utilities|Array|RemoveItem (Variables|Default|GetRopeList) _cable)
          (Actor|DestroyActor _cable))
        (:else
          _))
      (bind _pconstraint (Variables|/Game/GameProject2/Core/Characters/BP_RopePoints.BP_RopePoints_C|GetPConstraint _array_element)
        (:then
          (Actor|DestroyActor _pconstraint))
        (:else
          _))
      (if (== _array_element (Variables|Default|GetHit1))
        (Variables|Default|SetSecondShot false)
        (Variables|Default|SetCharge 0.0)
        (Variables|Default|SetChargePercent 0.0))
      (Game|SpawnActorfromClass "/Game/GameProject2/Core/Characters/BP_RetractProjectile.BP_RetractProjectile_C" (Math|Transform|MakeTransform (Transformation|GetWorldLocation (Variables|/Game/GameProject2/Core/Characters/BP_RopePoints.BP_RopePoints_C|GetDefaultSceneRoot _array_element)) "0, 0, 0" "1,1,1") "Undefined" 0 self 0)
      (Actor|DestroyActor _array_element)
      (Actor|GetAllActorsOfClass "/Script/CableComponent.CableActor")
      (Variables|Default|SetAmountOfLines 0)
      (Class|FMODBlueprintStatics|EventInstanceStop (stale _returnvalue))
      (bind _returnvalue (Class|FMODBlueprintStatics|PlayEvent2D "/Game/FMOD/Events/Player/Rope_Gun/Rope_Gun_Recall.Rope_Gun_Recall"))
      (switch int (Variables|Default|GetAmountOfLines)
        (:0
          (Rendering|SetVisibility (Variables|Default|GetStaticMesh4) true false))
        (:1
          (Rendering|SetVisibility (Variables|Default|GetStaticMesh3) true false))
        (:2
          (Rendering|SetVisibility (Variables|Default|GetStaticMesh2) true false))
        (:3
          (Rendering|SetVisibility (Variables|Default|GetStaticMesh1) true false))
        (:4
          (Rendering|SetVisibility (Variables|Default|GetStaticMesh) true false))))))

(event Custom|RetractAllPoints
  (bind _outactors (Actor|GetAllActorsOfClass "/Game/GameProject2/Core/Characters/BP_RopePoints.BP_RopePoints_C"))
  (for _array_element _outactors
    (Variables|/Game/GameProject2/Core/Characters/BP_RopePoints.BP_RopePoints_C|SetMarked _array_element true))
  (CallFunction|RemoveMarkedThings))

(event Custom|Ragdoll
  (bind _player_low (Variables|Default|GetPlayer_Low))
  ;[1 1 1] Ragdoll
  (Transformation|AttachComponentToComponent (Variables|Default|GetCameraBoom) (Variables|Default|GetPlayer_Low) "None" "KeepWorld" "KeepWorld" "KeepWorld" true)
  (for _index (range 0 1)
    (Class|SkeletalMeshComponent|SetAllBodiesSimulatePhysics _player_low true)
    (Collision|SetCollisionEnabled _player_low "QueryAndPhysics")))

(event Custom|OnDamageTaken_Event_0
  (params (Value :type Integer))
  ;[1 1 1] Damge take bind
  (Variables|/Script/GP2Team10Project.GP2Team10ProjectHealthComponent|SetbInvincible (Variables|Default|GetBP_HealthComponent) true)
  (Utilities|FlowControl|Sequence
    (:then_0
      (Utilities|ForLoopwithDelay 0 8 0.1
        (:LoopBody
          (Rendering|SetVisibility (Variables|Default|GetPlayer_Low) false false)
          (Utilities|FlowControl|Delay 0.1)
          (Rendering|SetVisibility (Variables|Default|GetPlayer_Low) true false))))
    (:then_1
      (Utilities|FlowControl|Delay 1.0)
      (Variables|/Script/GP2Team10Project.GP2Team10ProjectHealthComponent|SetbInvincible (Variables|Default|GetBP_HealthComponent) false))))

(event Custom|Event%20Pickup%20Triggered
  (Variables|Default|SetOverlapCount (+ (Variables|Default|GetOverlapCount) 1.0))
  ;[1 1 1] Event Pickup Triggered
  (Niagara|SpawnSystemAttached "/Game/GameProject2/Effects/Systems/HealthPickup.HealthPickup" (Variables|Default|GetParticleUpgrade) "None" "0, 0, 0" "0, 0, 0" "KeepRelativeOffset" true)
  (Variables|Default|SetParts (+ (Variables|Default|GetParts) 1))
  (if (and (== (Variables|Default|GetOverlapCount) 3.0) (<= (Class|GP2Team10ProjectHealthComponent|GetMaxHealth (Variables|Default|GetBP_HealthComponent)) 9))
    (Class|GP2Team10ProjectHealthComponent|ModifyMaxHealth (Variables|Default|GetBP_HealthComponent) (+ (Class|GP2Team10ProjectHealthComponent|GetMaxHealth (Variables|Default|GetBP_HealthComponent)) 1))
    (Niagara|SpawnSystemAttached "/Game/GameProject2/Effects/Systems/PS_HealthUpgrade.PS_HealthUpgrade" (Variables|Default|GetParticleUpgrade) "None" "0, 0, 0" "0, 0, 0" "KeepRelativeOffset" true)
    (Variables|Default|SetOverlapCount 0.0)))

(event Custom|Toggle
  (UserInterface|Viewport|AddtoViewport (Variables|Default|GetUI) 0))

(event EventBeginPlay
  ;[1 1 1] Initial checkpoint
  (bind _outactors (Actor|GetAllActorsOfClass "/Game/GameProject2/Placeables/BP_ShipwreckPart.BP_ShipwreckPart_C"))
  (Variables|Default|SetTargetLocation (Utilities|Array|Get(acopy) _outactors))
  (bind _returnvalue (UserInterface|CreateWidget "/Game/GameProject2/Core/Characters/W_ChargeBar.W_ChargeBar_C" (Game|GetPlayerController 0)))
  (Variables|Default|SetUI _returnvalue)
  (bind _asbp_gamemode (Utilities|Casting|CastToBP_Gamemode (Game|GetGameMode))
    (:then
      (EventDispatchers|BindEventtoToggleHUD _asbp_gamemode (delegate Custom|Toggle)))
    (:CastFailed
      _))
  ;[1 1 1] Damge take bind
  (EventDispatchers|AssignOnDamageTaken (Variables|Default|GetBP_HealthComponent) (delegate Custom|OnDamageTaken_Event_0)))

(event EventOnJumped
  (Variables|Default|SetJumped true)
  (Niagara|SpawnSystematLocation "/Game/GameProject2/Effects/Systems/PS_Jump.PS_Jump" (Transformation|GetWorldLocation (Variables|Default|GetJumpEffectLocation))))

(event EventOnLanded
  (params (Hit :type Hit%20Result%20Structure%20%28by%20ref%29))
  (Variables|Default|SetJumped false))

(event EventTick
  (params (DeltaSeconds :type Float%20%28single-precision%29))
  (bind _followcamera (Variables|Default|GetFollowCamera))
  (bind _returnvalue (Transformation|GetWorldLocation _followcamera))
  ;[1 1 1] Pil roterar mot nästa checkpoint
  (Utilities|FlowControl|Sequence
    (:then_1
      ;[1 1 1] Highlighting rope points
      (bind _outhits (Collision|MultiSphereTraceForObjects (+ (* (Math|Vector|GetForwardVector _followcamera) 1.5e+02) _returnvalue) (+ (* (Math|Vector|GetForwardVector _followcamera) 1e+04) _returnvalue) 1.5e+02 (Utilities|Array|MakeArray "ObjectTypeQuery7") true 0 "None"))
      (for _array_element _outhits
        (bind _asbp_rope_points (Utilities|Casting|CastToBP_RopePoints (.hitactor _array_element)))
        (Default|ToggleRed _asbp_rope_points)))
    (:then_2
      (if (Variables|Default|GetCharging)
        (if (<= (Variables|Default|GetCharge) 2.0)
          (Variables|Default|SetCharge (+ (Variables|Default|GetCharge) (Utilities|Time|GetWorldDeltaSeconds)))
          (Variables|Default|SetChargePercent (/ (Variables|Default|GetCharge) 2.0)))))
    (:then_3
      ;[1 1 1] Timer
      (if (Variables|Default|GetTimerOn)
        (bind _output_get (Variables|Default|SetTimer (+ (Variables|Default|GetTimer) DeltaSeconds)))
        (if (> _output_get 1.0)
          (CallFunction|RetractAllPoints))))))

(event EventOnThrust
  (bind _followcamera (Variables|Default|GetFollowCamera))
  (bind _cameraboom (Variables|Default|GetCameraBoom))
  (bind _followcamera_2 (Variables|Default|GetFollowCamera))
  (bind _returnvalue (Transformation|GetWorldLocation _cameraboom))
  (bind _returnvalue_2 (Transformation|GetWorldLocation _followcamera))
  (bind _returnvalue_3 (Math|Rotator|FindLookatRotation _returnvalue _returnvalue_2))
  ;[1 1 1] Air dash effect
  (Utilities|FlowControl|Sequence
    (:then_0
      (Utilities|FlowControl|Sequence
        (:then_0
          (bind _fovlerp (Timeline|Timeline_0 Stop)
            (:Update
              (Variables|/Script/Engine.CameraComponent|SetFieldOfView _followcamera_2 (+ (* _fovlerp -1.0) 9e+01)))))
        (:then_1
          (Variables|/Script/Engine.CameraComponent|SetFieldOfView _followcamera_2 9e+01))))
    (:then_1
      (Niagara|SpawnSystematLocation "/Game/GameProject2/Effects/Systems/PS_Thrust.PS_Thrust" (Transformation|GetWorldLocation (Variables|Default|GetScene)) (Math|Rotator|MakeRotator (.roll _returnvalue_3) (+ (.pitch _returnvalue_3) 9e+01) (.yaw _returnvalue_3))))))

(event Input|ActionEvents|InputActionShoot
  (params (Key :type Key%20Structure))
  (bind _shotexit (Variables|Default|GetShotExit))
  (bind _shotexit_2 (Variables|Default|GetShotExit))
  (bind _capsulecomponent (Variables|Default|GetCapsuleComponent))
  (bind _returnvalue (Transformation|GetWorldTransform _shotexit))
  (bind _returnvalue_2 (Transformation|GetWorldTransform _shotexit_2))
  (bind _returnvalue_3 (Transformation|GetWorldRotation _capsulecomponent))
  ;[1 1 1] Shoot Harpoon
  (:Pressed
    (if (< (Variables|Default|GetAmountOfLines) (Variables|Default|GetRopeMax))
      (if (Variables|Default|GetSecondShot)
        (Game|SpawnActorfromClass "/Game/GameProject2/Core/Characters/BP_PlayerHarpoon.BP_PlayerHarpoon_C" (Math|Transform|MakeTransform (.location _returnvalue_2) (.rotation _returnvalue_2) "2.000000,2.000000,2.000000") "Undefined" self "0.000000,0.000000,0.000000" 0)
        (else
          (Variables|Default|SetSecondShot true)
          (Utilities|FlowControl|Sequence
            (:then_0
              (Game|SpawnActorfromClass "/Game/GameProject2/Core/Characters/BP_PlayerHarpoon.BP_PlayerHarpoon_C" (Math|Transform|MakeTransform (.location _returnvalue) (.rotation _returnvalue) "2.000000,2.000000,2.000000") "Undefined" self "0.000000,0.000000,0.000000" 0)))))
      (Niagara|SpawnSystemAttached "/Game/GameProject2/Effects/Systems/PS_Shoot.PS_Shoot" (Variables|Default|GetPew) "" "0, 0, 0" "0, 0, 0" "KeepRelativeOffset" false)
      (Transformation|SetWorldRotation _capsulecomponent (Math|Rotator|MakeRotator (.roll _returnvalue_3) (.pitch _returnvalue_3) (.yaw (Class|SpringArmComponent|GetTargetRotation (Variables|Default|GetCameraBoom)))) false false)
      (Class|FMODBlueprintStatics|PlayEvent2D "/Game/FMOD/Events/Player/Rope_Gun/Rope_Gun_Fire.Rope_Gun_Fire")
      (Default|CallShoot))))

(event Input|ActionEvents|InputActionPause
  (params (Key :type Key%20Structure))
  ;[1 1 1] Pause game
  (:Pressed
    (CallFunction|PauseGame)))

(event Input|ActionEvents|InputActionRemove
  (params (Key :type Key%20Structure))
  (bind _followcamera (Variables|Default|GetFollowCamera))
  (bind _returnvalue (Transformation|GetWorldLocation _followcamera))
  (:Pressed
    (Variables|Default|SetTimer 0.0)
    (Variables|Default|SetTimerOn true))
  (:Released
    (Utilities|FlowControl|Sequence
      (:then_0
        (Variables|Default|SetTimerOn false)
        (if (< (Variables|Default|GetTimer) 1.0)
          ;[1 1 1] Rope deletion
          (bind _outhits (Collision|MultiSphereTraceForObjects (+ (* (Math|Vector|GetForwardVector _followcamera) 1.5e+02) _returnvalue) (+ (* (Math|Vector|GetForwardVector _followcamera) 1e+04) _returnvalue) 1.5e+02 (Utilities|Array|MakeArray "ObjectTypeQuery7") true 0 "None"))
          (for _array_element _outhits
            (bind _asbp_rope_points (Utilities|Casting|CastToBP_RopePoints (.hitactor _array_element)))
            (Variables|/Game/GameProject2/Core/Characters/BP_RopePoints.BP_RopePoints_C|SetMarked _asbp_rope_points true)
            (bind _otherhit (Variables|/Game/GameProject2/Core/Characters/BP_RopePoints.BP_RopePoints_C|GetOtherHit _asbp_rope_points)
              (:then
                (Variables|/Game/GameProject2/Core/Characters/BP_RopePoints.BP_RopePoints_C|SetMarked _otherhit true))
              (:else)))
          (CallFunction|RemoveMarkedThings))))))

(event Input|KeyboardEvents|Ö
  (params (Key :type Key%20Structure)))

(event Input|KeyboardEvents|LeftShift
  (params (Key :type Key%20Structure))
  (:Pressed
    (if (and (> (Variables|Default|GetThrustCharges) 0) (AI|Components|NavMovement|IsFalling (Variables|Character|GetCharacterMovement)))
      (Utilities|FlowControl|Sequence
        (:then_0
          (bind _fovlerp (Timeline|Timeline_0 PlayFromStart)
            (:Update
              (Variables|/Script/Engine.CameraComponent|SetFieldOfView (Variables|Default|GetFollowCamera) (+ (* _fovlerp -1.0) 9e+01)))))))))

(event Input|KeyboardEvents|H
  (params (Key :type Key%20Structure))
  (:Pressed
    (bind _asbp_gameinstance (Utilities|Casting|CastToBP_Gameinstance (Game|GetGameInstance)))
    (Default|RespawningPlayer _asbp_gameinstance)))

(event Input|KeyboardEvents|K
  (params (Key :type Key%20Structure))
  ;[1 1 1] TP to boss
  (:Pressed
    (bind _outactors (Actor|GetAllActorsOfClass "/Game/GameProject2/Core/Characters/BP_BossTP.BP_BossTP_C"))
    (Transformation|SetWorldLocation (Variables|Default|GetCapsuleComponent) (Transformation|GetWorldLocation (Variables|/Game/GameProject2/Core/Characters/BP_BossTP.BP_BossTP_C|GetDefaultSceneRoot (Utilities|Array|Get(acopy) _outactors))) false false)))

(event Input|KeyboardEvents|Ö
  (params (Key :type Key%20Structure))
  ;[1 1 1] TP to JesperLevel
  (:Pressed
    (bind _outactors (Actor|GetAllActorsOfClass "/Game/GameProject2/Core/Characters/BP_JesperTP.BP_JesperTP_C"))
    (Transformation|SetWorldLocation (Variables|Default|GetCapsuleComponent) (Transformation|GetWorldLocation (Variables|/Script/Engine.Actor|GetRootComponent (Utilities|Array|Get(acopy) _outactors))) false false)))

(event Input|KeyboardEvents|O
  (params (Key :type Key%20Structure))
  ;[1 1 1] TP to MalinLevel
  (:Pressed
    (bind _outactors (Actor|GetAllActorsOfClass "/Game/GameProject2/Core/Characters/BP_MalinTP.BP_MalinTP_C"))
    (Transformation|SetWorldLocation (Variables|Default|GetCapsuleComponent) (Transformation|GetWorldLocation (Variables|/Script/Engine.Actor|GetRootComponent (Utilities|Array|Get(acopy) _outactors))) false false)))

(fn ConstructionScript)

(fn PauseGame
  (bind _returnvalue (Game|GetPlayerController 0))
  ;[1 1 1] If it already automatically created the widget, we just add it to the viewport.
  (bind _returnvalue_2 (UserInterface|CreateWidget "/Game/GameProject2/Core/MenuUI/PauseMenu.PauseMenu_C" (Game|GetPlayerController 0)))
  (bind _output_get (Variables|Default|SetPauseMenu _returnvalue_2))
  (UserInterface|Viewport|AddtoViewport _output_get 0)
  (Utilities|Time|SetGlobalTimeDilation 0.01)
  (Input|SetInputModeUIOnly _returnvalue 0 "DoNotLock")
  (Variables|/Script/Engine.PlayerController|SetbShowMouseCursor _returnvalue true))

(fn UnpauseGame
  (bind _returnvalue (Game|GetPlayerController 0))
  (Utilities|Time|SetGlobalTimeDilation 1.0)
  (bind _foundwidgets (Widget|GetAllWidgetsOfClass "/Game/GameProject2/Core/MenuUI/PauseMenu.PauseMenu_C" true))
  (Widget|RemovefromParent _foundwidgets)
  (Input|SetInputModeGameOnly _returnvalue)
  (Variables|/Script/Engine.PlayerController|SetbShowMouseCursor _returnvalue false))

(fn DeathScreen
  ;[1 1 1] If it already automatically created the widget, we just add it to the viewport.
  (bind _returnvalue (UserInterface|CreateWidget "/Game/GameProject2/Core/MenuUI/W_DeathScreen.W_DeathScreen_C" (Game|GetPlayerController 0)))
  (UserInterface|Viewport|AddtoViewport _returnvalue 0))

(fn TutorialJumpPause
  (bind _returnvalue (Game|GetPlayerController 0))
  (bind _returnvalue_2 (UserInterface|CreateWidget "/Game/GameProject2/Core/MenuUI/JumpTutorialUI.JumpTutorialUI_C" (Game|GetPlayerController 0)))
  ;[1 1 1] If it already automatically created the widget, we just add it to the viewport.
  (bind _output_get (Variables|Default|Setuijump _returnvalue_2))
  (UserInterface|Viewport|AddtoViewport _output_get 0)
  (Utilities|Time|SetGlobalTimeDilation 0.01)
  (Input|SetInputModeUIOnly _returnvalue 0 "DoNotLock")
  (Variables|/Script/Engine.PlayerController|SetbShowMouseCursor _returnvalue true))

(fn TutorialUnpause
  (bind _returnvalue (Game|GetPlayerController 0))
  (Utilities|Time|SetGlobalTimeDilation 1.0)
  (Input|SetInputModeGameOnly _returnvalue)
  (Variables|/Script/Engine.PlayerController|SetbShowMouseCursor _returnvalue false))

(fn TutorialGlidePause
  (bind _returnvalue (Game|GetPlayerController 0))
  (bind _returnvalue_2 (UserInterface|CreateWidget "/Game/GameProject2/Core/MenuUI/GlideTutorialUI.GlideTutorialUI_C" (Game|GetPlayerController 0)))
  ;[1 1 1] If it already automatically created the widget, we just add it to the viewport.
  (bind _output_get (Variables|Default|Setuiglide _returnvalue_2))
  (UserInterface|Viewport|AddtoViewport _output_get 0)
  (Utilities|Time|SetGlobalTimeDilation 0.01)
  (Input|SetInputModeUIOnly _returnvalue 0 "DoNotLock")
  (Variables|/Script/Engine.PlayerController|SetbShowMouseCursor _returnvalue true))

(fn TutorialDashPause
  (bind _returnvalue (Game|GetPlayerController 0))
  (bind _returnvalue_2 (UserInterface|CreateWidget "/Game/GameProject2/Core/MenuUI/DashTutorialUI.DashTutorialUI_C" (Game|GetPlayerController 0)))
  (bind _output_get (Variables|Default|Setuidash _returnvalue_2))
  (UserInterface|Viewport|AddtoViewport _output_get 0)
  (Utilities|Time|SetGlobalTimeDilation 0.01)
  (Input|SetInputModeUIOnly _returnvalue 0 "DoNotLock")
  (Variables|/Script/Engine.PlayerController|SetbShowMouseCursor _returnvalue true))

(fn TutorialDashGlide
  (bind _returnvalue (Game|GetPlayerController 0))
  (bind _returnvalue_2 (UserInterface|CreateWidget "/Game/GameProject2/Core/MenuUI/DashGlideTutorialUI.DashGlideTutorialUI_C" (Game|GetPlayerController 0)))
  ;[1 1 1] If it already automatically created the widget, we just add it to the viewport.
  (bind _output_get (Variables|Default|Setuidashglide _returnvalue_2))
  (UserInterface|Viewport|AddtoViewport _output_get 0)
  (Utilities|Time|SetGlobalTimeDilation 0.01)
  (Input|SetInputModeUIOnly _returnvalue 0 "DoNotLock")
  (Variables|/Script/Engine.PlayerController|SetbShowMouseCursor _returnvalue true))

(fn TutorialTether
  (bind _returnvalue (Game|GetPlayerController 0))
  (bind _returnvalue_2 (UserInterface|CreateWidget "/Game/GameProject2/Core/MenuUI/TetherTutorialUI.TetherTutorialUI_C" (Game|GetPlayerController 0)))
  (bind _output_get (Variables|Default|Setuitether _returnvalue_2))
  (UserInterface|Viewport|AddtoViewport _output_get 0)
  (Utilities|Time|SetGlobalTimeDilation 0.01)
  (Input|SetInputModeUIOnly _returnvalue 0 "DoNotLock")
  (Variables|/Script/Engine.PlayerController|SetbShowMouseCursor _returnvalue true))