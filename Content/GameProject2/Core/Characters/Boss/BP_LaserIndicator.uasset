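; BP_LaserIndicator is a laser indicator for a boss attack that can damage the player.
; Its Fire event makes the Cylinder and LASER components visible, then does a single overlap test of LASER against the Player and calls DealDamage on the Boss if they overlap.
; The LASER begin-overlap event is empty, and an older-style player check leading to DealDamage sits disconnected, so damage only happens at the moment of firing.
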(event OnComponentBeginOverlap(LASER)
  (params (OverlappedComponent :type Primitive%20Component%20Object%20Reference) (OtherActor :type Actor%20Object%20Reference) (OtherComp :type Primitive%20Component%20Object%20Reference) (OtherBodyIndex :type Integer) (bFromSweep :type Boolean) (SweepResult :type Hit%20Result%20Structure%20%28by%20ref%29)))

(event Custom|Fire
  (Rendering|SetVisibility (Variables|Default|GetCylinder) true false)
  (if (Collision|IsOverlappingActor (Variables|Default|GetLASER) (Variables|Default|GetPlayer) :!class /Script/Engine.PrimitiveComponent)
    (Default|DealDamage (Variables|Default|GetBoss))))

(fn ConstructionScript)