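; Boss bramble wall hazard that sweeps along world -X and destroys itself near a point 5000 units from its spawn.
; Each tick, three base components lerp around their own four-marker loops, advancing a state counter on arrival within tolerance, while the root moves at Speed.
; Hitbox overlap with the player pawn deals 1 damage and launches them away from the wall's root.
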(event OnComponentBeginOverlap(Hitbox)
  (params (OverlappedComponent :type Primitive%20Component%20Object%20Reference) (OtherActor :type Actor%20Object%20Reference) (OtherComp :type Primitive%20Component%20Object%20Reference) (OtherBodyIndex :type Integer) (bFromSweep :type Boolean) (SweepResult :type Hit%20Result%20Structure%20%28by%20ref%29))
  (bind _asbp_player_pawn (Utilities|Casting|CastToBP_PlayerPawn OtherActor))
  (Utilities|FlowControl|DoOnce false :!label _label
    (:Completed
      (Class|GP2Team10ProjectHealthComponent|DecreaseHealth (Variables|/Game/GameProject2/Core/Characters/BP_PlayerPawn.BP_PlayerPawn_C|GetBP_HealthComponent _asbp_player_pawn) 1)
      (Character|LaunchCharacter _asbp_player_pawn (* (Math|Vector|Normalize (- (Transformation|GetWorldLocation (Variables|/Script/Engine.Character|GetCapsuleComponent _asbp_player_pawn)) (Transformation|GetWorldLocation (Variables|Default|GetDefaultSceneRoot)))) 2.5e+03) false false)
      (goto _label Reset))))

(event EventTick
  (params (DeltaSeconds :type Float%20%28single-precision%29))
  (bind _base2 (Variables|Default|GetBase2))
  (bind _scene8 (Variables|Default|GetScene8))
  (bind _base2_2 (Variables|Default|GetBase2))
  (bind _scene9 (Variables|Default|GetScene9))
  (bind _base3 (Variables|Default|GetBase3))
  (bind _rotationlocation1 (Variables|Default|GetRotationlocation1))
  (bind _scene10 (Variables|Default|GetScene10))
  (bind _base3_2 (Variables|Default|GetBase3))
  (bind _scene (Variables|Default|GetScene))
  (bind _base3_3 (Variables|Default|GetBase3))
  (bind _scene1 (Variables|Default|GetScene1))
  (bind _base3_4 (Variables|Default|GetBase3))
  (bind _base2_3 (Variables|Default|GetBase2))
  (bind _scene2 (Variables|Default|GetScene2))
  (bind _base1 (Variables|Default|GetBase1))
  (bind _scene6 (Variables|Default|GetScene6))
  (bind _base1_2 (Variables|Default|GetBase1))
  (bind _scene5 (Variables|Default|GetScene5))
  (bind _base1_3 (Variables|Default|GetBase1))
  (bind _scene4 (Variables|Default|GetScene4))
  (bind _base1_4 (Variables|Default|GetBase1))
  (bind _scene3 (Variables|Default|GetScene3))
  (bind _base2_4 (Variables|Default|GetBase2))
  (bind _scene7 (Variables|Default|GetScene7))
  (bind _returnvalue (Transformation|GetWorldLocation _base2))
  (bind _returnvalue_2 (Transformation|GetWorldLocation _scene8))
  (bind _returnvalue_3 (Transformation|GetWorldLocation _base2_2))
  (bind _returnvalue_4 (Transformation|GetWorldLocation _scene9))
  (bind _returnvalue_5 (Transformation|GetWorldLocation _base3))
  (bind _returnvalue_6 (Transformation|GetWorldLocation _rotationlocation1))
  (bind _returnvalue_7 (Transformation|GetWorldLocation _base3_2))
  (bind _returnvalue_8 (Transformation|GetWorldLocation _scene))
  (bind _returnvalue_9 (Transformation|GetWorldLocation _scene10))
  (bind _returnvalue_10 (Transformation|GetWorldLocation _base3_3))
  (bind _returnvalue_11 (Transformation|GetWorldLocation _scene1))
  (bind _returnvalue_12 (Transformation|GetWorldLocation _base3_4))
  (bind _returnvalue_13 (Transformation|GetWorldLocation _scene2))
  (bind _returnvalue_14 (Transformation|GetWorldLocation _base2_3))
  (bind _returnvalue_15 (Transformation|GetWorldLocation _base1))
  (bind _returnvalue_16 (Transformation|GetWorldLocation _scene6))
  (bind _returnvalue_17 (Transformation|GetWorldLocation _base1_2))
  (bind _returnvalue_18 (Transformation|GetWorldLocation _scene5))
  (bind _returnvalue_19 (Transformation|GetWorldLocation _base1_3))
  (bind _returnvalue_20 (Transformation|GetWorldLocation _scene4))
  (bind _returnvalue_21 (Transformation|GetWorldLocation _base1_4))
  (bind _returnvalue_22 (Transformation|GetWorldLocation _scene3))
  (bind _returnvalue_23 (Transformation|GetWorldLocation _base2_4))
  (bind _returnvalue_24 (Transformation|GetWorldLocation _scene7))
  (Utilities|FlowControl|Sequence
    (:then_0
      (switch int (Variables|Default|GetRotationHandler)
        (:0
          (Transformation|SetWorldLocation (Variables|Default|GetBase3) (Math|Vector|Lerp(Vector) _returnvalue_5 _returnvalue_6 (Variables|Default|GetRotationSpeed)) false false)
          (if (Math|Vector|Equal(Vector) _returnvalue_5 _returnvalue_6 (Variables|Default|GetErrorTolerance))
            (Math|Integer|IncrementInt (Variables|Default|GetRotationHandler))))
        (:1
          (Transformation|SetWorldLocation (Variables|Default|GetBase3) (Math|Vector|Lerp(Vector) _returnvalue_7 _returnvalue_8 (Variables|Default|GetRotationSpeed)) false false)
          (if (Math|Vector|Equal(Vector) _returnvalue_7 _returnvalue_8 (Variables|Default|GetErrorTolerance))
            (Math|Integer|IncrementInt (Variables|Default|GetRotationHandler))))
        (:2
          (Transformation|SetWorldLocation (Variables|Default|GetBase3) (Math|Vector|Lerp(Vector) _returnvalue_10 _returnvalue_11 (Variables|Default|GetRotationSpeed)) false false)
          (if (Math|Vector|Equal(Vector) _returnvalue_10 _returnvalue_11 (Variables|Default|GetErrorTolerance))
            (Math|Integer|IncrementInt (Variables|Default|GetRotationHandler))))
        (:3
          (Transformation|SetWorldLocation (Variables|Default|GetBase3) (Math|Vector|Lerp(Vector) _returnvalue_12 _returnvalue_13 (Variables|Default|GetRotationSpeed)) false false)
          (if (Math|Vector|Equal(Vector) _returnvalue_12 _returnvalue_13 (Variables|Default|GetErrorTolerance))
            (Variables|Default|SetRotationHandler 0)))))
    (:then_1
      (switch int (Variables|Default|GetRotationHandler2)
        (:0
          (Transformation|SetWorldLocation (Variables|Default|GetBase1) (Math|Vector|Lerp(Vector) _returnvalue_15 _returnvalue_16 (Variables|Default|GetRotationSpeed)) false false)
          (if (Math|Vector|Equal(Vector) _returnvalue_15 _returnvalue_16 (Variables|Default|GetErrorTolerance))
            (Math|Integer|IncrementInt (Variables|Default|GetRotationHandler2))))
        (:1
          (Transformation|SetWorldLocation (Variables|Default|GetBase1) (Math|Vector|Lerp(Vector) _returnvalue_17 _returnvalue_18 (Variables|Default|GetRotationSpeed)) false false)
          (if (Math|Vector|Equal(Vector) _returnvalue_17 _returnvalue_18 (Variables|Default|GetErrorTolerance))
            (Math|Integer|IncrementInt (Variables|Default|GetRotationHandler2))))
        (:2
          (Transformation|SetWorldLocation (Variables|Default|GetBase1) (Math|Vector|Lerp(Vector) _returnvalue_19 _returnvalue_20 (Variables|Default|GetRotationSpeed)) false false)
          (if (Math|Vector|Equal(Vector) _returnvalue_19 _returnvalue_20 (Variables|Default|GetErrorTolerance))
            (Math|Integer|IncrementInt (Variables|Default|GetRotationHandler2))))
        (:3
          (Transformation|SetWorldLocation (Variables|Default|GetBase1) (Math|Vector|Lerp(Vector) _returnvalue_21 _returnvalue_22 (Variables|Default|GetRotationSpeed)) false false)
          (if (Math|Vector|Equal(Vector) _returnvalue_21 _returnvalue_22 (Variables|Default|GetErrorTolerance))
            (Variables|Default|SetRotationHandler2 0)))))
    (:then_2
      (switch int (Variables|Default|GetRotationHandler3)
        (:0
          (Transformation|SetWorldLocation (Variables|Default|GetBase2) (Math|Vector|Lerp(Vector) _returnvalue_23 _returnvalue_24 (Variables|Default|GetRotationSpeed)) false false)
          (if (Math|Vector|Equal(Vector) _returnvalue_23 _returnvalue_24 (Variables|Default|GetErrorTolerance))
            (Math|Integer|IncrementInt (Variables|Default|GetRotationHandler3))))
        (:1
          (Transformation|SetWorldLocation (Variables|Default|GetBase2) (Math|Vector|Lerp(Vector) _returnvalue _returnvalue_2 (Variables|Default|GetRotationSpeed)) false false)
          (if (Math|Vector|Equal(Vector) _returnvalue _returnvalue_2 (Variables|Default|GetErrorTolerance))
            (Math|Integer|IncrementInt (Variables|Default|GetRotationHandler3))))
        (:2
          (Transformation|SetWorldLocation (Variables|Default|GetBase2) (Math|Vector|Lerp(Vector) _returnvalue_3 _returnvalue_4 (Variables|Default|GetRotationSpeed)) false false)
          (if (Math|Vector|Equal(Vector) _returnvalue_3 _returnvalue_4 (Variables|Default|GetErrorTolerance))
            (Math|Integer|IncrementInt (Variables|Default|GetRotationHandler3))))
        (:3
          (Transformation|SetWorldLocation (Variables|Default|GetBase2) (Math|Vector|Lerp(Vector) _returnvalue_14 _returnvalue_9 (Variables|Default|GetRotationSpeed)) false false)
          (if (Math|Vector|Equal(Vector) _returnvalue_14 _returnvalue_9 (Variables|Default|GetErrorTolerance))
            (Variables|Default|SetRotationHandler3 0)))))
    (:then_3
      (Transformation|AddWorldOffset (Variables|Default|GetDefaultSceneRoot) (Math|Vector|MakeVector (* (* (Variables|Default|GetSpeed) -1.0) (Utilities|Time|GetWorldDeltaSeconds)) 0.0 0.0) false false)
      (if (Math|Vector|Equal(Vector) (Transformation|GetWorldLocation (Variables|Default|GetDefaultSceneRoot)) (Variables|Default|GetTarget) 1e+01)
        (Actor|DestroyActor)))))

(event EventBeginPlay
  (bind _defaultsceneroot (Variables|Default|GetDefaultSceneRoot))
  (bind _returnvalue (Transformation|GetWorldLocation _defaultsceneroot))
  (Variables|Default|SetTarget (Math|Vector|MakeVector (- (.x _returnvalue) 5e+03) (.y _returnvalue) (.z _returnvalue))))

(fn ConstructionScript)