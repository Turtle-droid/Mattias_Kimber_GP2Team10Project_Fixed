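; BP_ShockWave is an expanding shockwave actor for a boss that damages the player on contact.
; Each tick it widens its Cylinder uniformly in X and Y at ScaleIncreaseRate with a fixed height, then destroys itself past a maximum width.
; When the Player begins overlapping the Cylinder, it calls DealDamage on the Boss reference rather than applying damage itself.
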(event OnComponentBeginOverlap(Cylinder)
  (params (OverlappedComponent :type Primitive%20Component%20Object%20Reference) (OtherActor :type Actor%20Object%20Reference) (OtherComp :type Primitive%20Component%20Object%20Reference) (OtherBodyIndex :type Integer) (bFromSweep :type Boolean) (SweepResult :type Hit%20Result%20Structure%20%28by%20ref%29))
  (if (== (Variables|Default|GetPlayer) OtherActor)
    (Default|DealDamage (Variables|Default|GetBoss))))

(event EventTick
  (params (DeltaSeconds :type Float%20%28single-precision%29))
  (bind _cylinder (Variables|Default|GetCylinder))
  (bind _scaleincreaserate (Variables|Default|GetScaleIncreaseRate))
  (bind _returnvalue (Transformation|GetWorldScale _cylinder))
  (bind _returnvalue_2 (* DeltaSeconds _scaleincreaserate))
  (bind _returnvalue_3 (+ (.x _returnvalue) _returnvalue_2))
  (Transformation|SetWorldScale3D _cylinder (Math|Vector|MakeVector _returnvalue_3 _returnvalue_3 15.0))
  (if (> (.x _returnvalue) 7e+01)
    (Actor|DestroyActor)))

(fn ConstructionScript)