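; BP_Bosspit is a hazard actor, named as a boss pit, that damages the player on contact and throws them clear.
; On BeginPlay it caches player 0's controlled pawn as a BP_PlayerPawn.
; When that pawn overlaps it, the actor removes one point through BPHealthComponent and calls LaunchCharacter with a fixed up-and-negative-Y velocity that overrides current movement.
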(event EventBeginPlay
  (bind _asbp_player_pawn (Utilities|Casting|CastToBP_PlayerPawn (Pawn|GetControlledPawn (Game|GetPlayerController 0))))
  (Variables|Default|SetPlayer _asbp_player_pawn))

(event Collision|EventActorBeginOverlap
  (params (OtherActor :type Actor%20Object%20Reference))
  (bind _player (Variables|Default|GetPlayer))
  (if (== OtherActor (Variables|Default|GetPlayer))
    (Class|GP2Team10ProjectHealthComponent|DecreaseHealth (Variables|/Game/GameProject2/Core/Characters/BP_PlayerPawn.BP_PlayerPawn_C|GetBP_HealthComponent _player) 1)
    (Character|LaunchCharacter _player "0,-1000.000000,1000.000000" true true)))

(fn ConstructionScript)