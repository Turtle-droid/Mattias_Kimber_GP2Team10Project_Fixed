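; BP_Boss is a boss that activates with a camera-shake intro when the player enters its box, then faces and attacks them.
; A timed loop forces a short attack every third turn, otherwise making distance-weighted rolls with repeat limits.
; Attacks are shockwaves with enemy spawns, spinning bramble walls and telegraphed lasers.
; Body contact damages and launches the player; boss hits flicker eyes and crack the crystal, until death triggers the win.
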(event OnComponentBeginOverlap(Box)
  (params (OverlappedComponent :type Primitive%20Component%20Object%20Reference) (OtherActor :type Actor%20Object%20Reference) (OtherComp :type Primitive%20Component%20Object%20Reference) (OtherBodyIndex :type Integer) (bFromSweep :type Boolean) (SweepResult :type Hit%20Result%20Structure%20%28by%20ref%29))
  (bind _returnvalue (Game|GetPlayerController 0))
  (bind _returnvalue_2 (Game|GetPlayerController 0))
  (if (== OtherActor (Variables|Default|GetPlayer))
    (Utilities|FlowControl|DoOnce false
      (:Completed
        (Variables|Default|SetPlayIntro true)
        (Input|DisableInput (Pawn|GetControlledPawn _returnvalue) _returnvalue)
        (bind _returnvalue_3 (Utilities|Time|SetTimerbyEvent (EventDispatchers|CreateEvent :!event Custom|LookAtBoss) 0.001 true))
        (Variables|Default|SetLookAt _returnvalue_3)
        (Utilities|FlowControl|Delay 1.0)
        (Class|PlayerController|ClientPlayCameraShake _returnvalue_2 "/Game/GameProject2/Core/Characters/Boss/BP_Camerashake.BP_Camerashake_C" 1.0 "CameraLocal" "0, 0, 0")
        (Utilities|FlowControl|Sequence
          (:then_0
            (Utilities|FlowControl|Delay 2.0)
            (Input|EnableInput _returnvalue_2 _returnvalue_2)
            (Utilities|Time|PauseTimerbyHandle (Variables|Default|GetLookAt))
            (Variables|Default|SetBossActive true)
            (Variables|Default|SetPlayIntro false)
            (CallFunction|StartAtacking))
          (:then_1
            (Class|FMODBlueprintStatics|PlayEventAttached "/Game/FMOD/Events/Enemies/Boss/Boss_Vocal/Boss_Taunt.Boss_Taunt" (Variables|Default|GetSkeletalMesh) "None" "0, 0, 0" "KeepRelativeOffset")))))))

(event OnComponentBeginOverlap(Hand)
  (params (OverlappedComponent :type Primitive%20Component%20Object%20Reference) (OtherActor :type Actor%20Object%20Reference) (OtherComp :type Primitive%20Component%20Object%20Reference) (OtherBodyIndex :type Integer) (bFromSweep :type Boolean) (SweepResult :type Hit%20Result%20Structure%20%28by%20ref%29))
  ;[1 1 1] Character hit
  (if (== OtherActor (Variables|Default|GetPlayer))
    (Utilities|FlowControl|DoOnce false :!label _label
      (:Completed
        (CallFunction|DealDamage)
        (Utilities|FlowControl|Delay 1.0)
        (goto _label Reset)))))

(event OnComponentEndOverlap(Box)
  (params (OverlappedComponent :type Primitive%20Component%20Object%20Reference) (OtherActor :type Actor%20Object%20Reference) (OtherComp :type Primitive%20Component%20Object%20Reference) (OtherBodyIndex :type Integer))
  (bind _returnvalue (Game|GetPlayerController 0))
  (bind _returnvalue_2 (Game|GetPlayerController 0))
  (if (== OtherActor (Variables|Default|GetPlayer))
    (Variables|Default|SetBossActive false)
    (Utilities|FlowControl|Sequence
      (:then_0
        (Utilities|ForLoopwithDelay 0 100 1e+01) ; enters at Break
      )
      (:then_1
        (Utilities|FlowControl|DoOnce false) ; enters at Reset
      ))))

(event OnComponentBeginOverlap(Arm)
  (params (OverlappedComponent :type Primitive%20Component%20Object%20Reference) (OtherActor :type Actor%20Object%20Reference) (OtherComp :type Primitive%20Component%20Object%20Reference) (OtherBodyIndex :type Integer) (bFromSweep :type Boolean) (SweepResult :type Hit%20Result%20Structure%20%28by%20ref%29))
  ;[1 1 1] Character hit
  (if (== OtherActor (Variables|Default|GetPlayer))
    (Utilities|FlowControl|DoOnce false :!label _label
      (:Completed
        (CallFunction|DealDamage)
        (Utilities|FlowControl|Delay 1.0)
        (goto _label Reset)))))

(event OnComponentBeginOverlap(Hand2)
  (params (OverlappedComponent :type Primitive%20Component%20Object%20Reference) (OtherActor :type Actor%20Object%20Reference) (OtherComp :type Primitive%20Component%20Object%20Reference) (OtherBodyIndex :type Integer) (bFromSweep :type Boolean) (SweepResult :type Hit%20Result%20Structure%20%28by%20ref%29))
  ;[1 1 1] Character hit
  (if (== OtherActor (Variables|Default|GetPlayer))
    (Utilities|FlowControl|DoOnce false :!label _label
      (:Completed
        (CallFunction|DealDamage)
        (Utilities|FlowControl|Delay 1.0)
        (goto _label Reset)))))

(event OnComponentBeginOverlap(Arm2)
  (params (OverlappedComponent :type Primitive%20Component%20Object%20Reference) (OtherActor :type Actor%20Object%20Reference) (OtherComp :type Primitive%20Component%20Object%20Reference) (OtherBodyIndex :type Integer) (bFromSweep :type Boolean) (SweepResult :type Hit%20Result%20Structure%20%28by%20ref%29))
  ;[1 1 1] Character hit
  (if (== OtherActor (Variables|Default|GetPlayer))
    (Utilities|FlowControl|DoOnce false :!label _label
      (:Completed
        (CallFunction|DealDamage)
        (Utilities|FlowControl|Delay 1.0)
        (goto _label Reset)))))

(event OnComponentBeginOverlap(Body)
  (params (OverlappedComponent :type Primitive%20Component%20Object%20Reference) (OtherActor :type Actor%20Object%20Reference) (OtherComp :type Primitive%20Component%20Object%20Reference) (OtherBodyIndex :type Integer) (bFromSweep :type Boolean) (SweepResult :type Hit%20Result%20Structure%20%28by%20ref%29))
  ;[1 1 1] Character hit
  (if (== OtherActor (Variables|Default|GetPlayer))
    (Utilities|FlowControl|DoOnce false :!label _label
      (:Completed
        (CallFunction|DealDamage)
        (Utilities|FlowControl|Delay 1.0)
        (goto _label Reset)))))

(event OnComponentBeginOverlap(Head)
  (params (OverlappedComponent :type Primitive%20Component%20Object%20Reference) (OtherActor :type Actor%20Object%20Reference) (OtherComp :type Primitive%20Component%20Object%20Reference) (OtherBodyIndex :type Integer) (bFromSweep :type Boolean) (SweepResult :type Hit%20Result%20Structure%20%28by%20ref%29))
  ;[1 1 1] Character hit
  (if (== OtherActor (Variables|Default|GetPlayer))
    (Utilities|FlowControl|DoOnce false :!label _label
      (:Completed
        (CallFunction|DealDamage)
        (Utilities|FlowControl|Delay 1.0)
        (goto _label Reset)))))

(event Custom|Start%20Atacking
  (bind _index (Utilities|ForLoopwithDelay 0 100 1e+01)
    (:LoopBody
      (if (== (/ (Math|Conversions|ToFloat(Integer) _index) 3.0) (Math|Conversions|ToFloat(Integer) (Math|Float|Round (/ (Math|Conversions|ToFloat(Integer) _index) 3.0))))
        (CallFunction|ShortRangeAttack)
        (else
          (Variables|Default|SetAttackRoll (Math|Random|RandomFloatinRange 0.0 1e+02) :!label _label)
          (switch int (Variables|Default|GetRangeInt)
            (:0
              (if (<= (Variables|Default|GetAttackRoll) 1e+01)
                (if (!= (Variables|Default|GetLongOdds) 2)
                  (CallFunction|LongRangeAttack)
                  (Math|Integer|IncrementInt (Variables|Default|GetLongOdds)
                    (:%20%20
                      (Variables|Default|SetMidOdds 0)
                      (Variables|Default|SetShortOdds 0)))
                  (else
                    (goto _label)))
                (elif (Math|Float|InRange(Float) (Variables|Default|GetAttackRoll) 1e+01 3e+01 false)
                  (if (!= (Variables|Default|GetMidOdds) 2)
                    (CallFunction|MidRangeAttack)
                    (Math|Integer|IncrementInt (Variables|Default|GetMidOdds)
                      (:%20%20
                        (Variables|Default|SetLongOdds 0)
                        (Variables|Default|SetShortOdds 0)))
                    (else
                      (goto _label)))
                  (elif (!= (Variables|Default|GetShortOdds) 0)
                    (CallFunction|ShortRangeAttack)
                    (Math|Integer|IncrementInt (Variables|Default|GetShortOdds)
                      (:%20%20
                        (Variables|Default|SetLongOdds 0)
                        (Variables|Default|SetMidOdds 0)))
                    (else
                      (goto _label))))))
            (:1
              (if (<= (Variables|Default|GetAttackRoll) 2e+01)
                (if (!= (Variables|Default|GetLongOdds) 2)
                  (CallFunction|LongRangeAttack)
                  (Math|Integer|IncrementInt (Variables|Default|GetLongOdds)
                    (:%20%20
                      (Variables|Default|SetMidOdds 0)
                      (Variables|Default|SetShortOdds 0)))
                  (else
                    (goto _label)))
                (elif (Math|Float|InRange(Float) (Variables|Default|GetAttackRoll) 2e+01 8e+01 false)
                  (if (!= (Variables|Default|GetMidOdds) 2)
                    (CallFunction|MidRangeAttack)
                    (Math|Integer|IncrementInt (Variables|Default|GetMidOdds)
                      (:%20%20
                        (Variables|Default|SetLongOdds 0)
                        (Variables|Default|SetShortOdds 0)))
                    (else
                      (goto _label)))
                  (elif (!= (Variables|Default|GetShortOdds) 2)
                    (CallFunction|ShortRangeAttack)
                    (Math|Integer|IncrementInt (Variables|Default|GetShortOdds)
                      (:%20%20
                        (Variables|Default|SetLongOdds 0)
                        (Variables|Default|SetMidOdds 0)))
                    (else
                      (goto _label))))))
            (:2
              (if (<= (Variables|Default|GetAttackRoll) 7e+01)
                (if (!= (Variables|Default|GetLongOdds) 2)
                  (CallFunction|LongRangeAttack)
                  (Math|Integer|IncrementInt (Variables|Default|GetLongOdds)
                    (:%20%20
                      (Variables|Default|SetMidOdds 0)
                      (Variables|Default|SetShortOdds 0)))
                  (else
                    (goto _label)))
                (elif (Math|Float|InRange(Float) (Variables|Default|GetAttackRoll) 7e+01 9e+01 false)
                  (if (!= (Variables|Default|GetMidOdds) 2)
                    (CallFunction|MidRangeAttack)
                    (Math|Integer|IncrementInt (Variables|Default|GetMidOdds)
                      (:%20%20
                        (Variables|Default|SetLongOdds 0)
                        (Variables|Default|SetShortOdds 0)))
                    (else
                      (goto _label)))
                  (elif (!= (Variables|Default|GetShortOdds) 2)
                    (CallFunction|ShortRangeAttack)
                    (Math|Integer|IncrementInt (Variables|Default|GetShortOdds)
                      (:%20%20
                        (Variables|Default|SetLongOdds 0)
                        (Variables|Default|SetMidOdds 0)))
                    (else
                      (goto _label))))))))))))

(event Custom|LongRangeAttack
  (bind _crystalhitbox (Variables|Default|GetCrystalHitbox))
  ;[1 1 1] Long range attack
  (Variables|Default|SetIsLongRangeAttack true)
  (Utilities|FlowControl|Delay 2.2)
  (Variables|Default|SetIsAttacking true)
  (bind _returnvalue (Game|SpawnActorfromClass "/Game/GameProject2/Core/Characters/Boss/BP_LaserIndicator.BP_LaserIndicator_C" (Math|Transform|MakeTransform (Transformation|GetWorldLocation _crystalhitbox) (Math|Rotator|FindLookatRotation (Transformation|GetWorldLocation _crystalhitbox) (Transformation|GetWorldLocation (Variables|/Script/Engine.Character|GetCapsuleComponent (Variables|Default|GetPlayer))))) "Undefined" 0 (Variables|Default|GetPlayer) self 0))
  (bind _output_get (Variables|Default|SetLaserIndicator _returnvalue))
  (Utilities|FlowControl|Delay 1.0)
  (Default|Fire _output_get)
  (Utilities|FlowControl|Delay 1.4)
  (Actor|DestroyActor (Variables|Default|GetLaserIndicator))
  (Utilities|FlowControl|Delay 1.0)
  (Variables|Default|SetIsLongRangeAttack false)
  (Variables|Default|SetIsAttacking false))

(event Custom|MidRangeAttack
  ;[1 1 1] Medium Range attack
  (Variables|Default|SetIsMediumRangeAttack true)
  (Variables|Default|SetIsAttacking true)
  (Utilities|FlowControl|Delay 2.5)
  (Game|SpawnActorfromClass "/Game/GameProject2/Core/Characters/Boss/BP_BrambleWallSpinning.BP_BrambleWallSpinning_C" (Transformation|GetWorldTransform (Variables|/Game/GameProject2/Core/Characters/Boss/BP_BrambleSpawn.BP_BrambleSpawn_C|GetDefaultSceneRoot (Variables|Default|GetBrambleSpawn))) "Undefined" 0 0)
  (Utilities|FlowControl|Delay 1.5)
  (Variables|Default|SetIsMediumRangeAttack false)
  (Variables|Default|SetIsAttacking false))

(event Custom|ShortRangeAttack
  (bind _hand2 (Variables|Default|GetHand2))
  (bind _returnvalue (Transformation|GetWorldLocation _hand2))
  ;[1 1 1] Short range attack
  (Variables|Default|SetIsShortRangeAttack true)
  (Variables|Default|SetEnemySpawnIndex 0)
  (Utilities|ForLoopwithDelay 0 2 2.5
    (:LoopBody
      (Utilities|FlowControl|Delay 1.7)
      (bind (_outhit _returnvalue_2) (Collision|LineTraceByChannel (Transformation|GetWorldLocation _hand2) (Math|Vector|MakeVector (.x _returnvalue) (.y _returnvalue) (- (.z _returnvalue) 9e+03)) "TraceTypeQuery1" true 0 "None"))
      (if _returnvalue_2
        (Game|SpawnActorfromClass "/Game/GameProject2/Core/Characters/Boss/BP_ShockWave.BP_ShockWave_C" (Math|Transform|MakeTransform (.location _outhit) "0, 0, 0" "5.000000,5.000000,5.000000") "Undefined" 0 self (Variables|Default|GetPlayer) 0)
        (Default|SpwanEnemy (Utilities|Array|Get(acopy) (Variables|Default|GetSpawnLocations) (Variables|Default|GetEnemySpawnIndex)))
        (Math|Integer|IncrementInt (Variables|Default|GetEnemySpawnIndex))))
    (:Completed
      (Variables|Default|SetIsShortRangeAttack false))))

(event Custom|BossTakeDmg
  ;[1 1 1] Boss take damage
  (Niagara|SpawnSystematLocation "/Game/GameProject2/Effects/Systems/PS_Boss_Damage_FX.PS_Boss_Damage_FX" (Transformation|GetWorldLocation (Variables|Default|GetCrystalHitbox)))
  (bind _output_get (Variables|Default|SetHealth (- (Variables|Default|GetHealth) 1.0)))
  (Utilities|FlowControl|Sequence
    (:then_0
      (if (> _output_get 0.0)
        (Variables|Default|SetIsTakingDamage true)
        (Utilities|ForLoopwithDelay 0 4 0.1
          (:LoopBody
            (Rendering|Material|SetScalarParameterValueonMaterials (Variables|Default|GetEye1) "Opacity" 0.0)
            (Utilities|FlowControl|Delay 0.2)
            (Rendering|Material|SetScalarParameterValueonMaterials (Variables|Default|GetEye1) "Opacity" 1.0))
          (:Completed
            (Variables|Default|SetIsTakingDamage false)))
        (else
          (Variables|Default|SetIsAttacking false)
          (Utilities|ForLoopwithDelay 0 7 0.3
            (:LoopBody
              (Utilities|FlowControl|Delay 0.2))
            (:Completed
              (bind _asbp_gamemode (Utilities|Casting|CastToBP_Gamemode (Game|GetGameMode)))
              (Default|PlayerWin _asbp_gamemode)
              (Actor|DestroyActor))))))
    (:then_1
      (if (== (Variables|Default|GetHealth) 3.0)
        (Rendering|Material|SetMaterial (Variables|Default|GetCrystal) 0 "/Game/GameProject2/Effects/FXAssets/MI_New_Boss_Crystal_Cracked.MI_New_Boss_Crystal_Cracked"))
      (if (== (Variables|Default|GetHealth) 0.0)
        (Rendering|Material|SetMaterial (Variables|Default|GetCrystal) 0 "/Game/GameProject2/Effects/FXAssets/MI_New_Boss_Crystal_Dead.MI_New_Boss_Crystal_Dead")
        (Rendering|Material|SetScalarParameterValueonMaterials (Variables|Default|GetEye1) "Opacity" 0.0)))))

(event Custom|Death
  (Default|Ragdoll (Variables|Default|GetPlayer))
  (Utilities|Time|SetGlobalTimeDilation 0.2)
  (Default|DeathScreen (Variables|Default|GetPlayer)))

(event Custom|ResetBoss
  (bind _returnvalue (Game|GetPlayerController 0))
  (bind _returnvalue_2 (Game|GetPlayerController 0))
  (Variables|Default|SetHealth (Variables|Default|GetMaxHealth))
  (Variables|Default|SetBossActive false)
  (Utilities|FlowControl|Sequence
    (:then_0
      (Utilities|ForLoopwithDelay 0 100 1e+01) ; enters at Break
    )
    (:then_1
      (Utilities|FlowControl|DoOnce false) ; enters at Reset
    )))

(event Custom|Deal%20damage
  (bind _player (Variables|Default|GetPlayer))
  (bind _player_2 (Variables|Default|GetPlayer))
  (bind _staticmeshcomponent (Variables|Debug|GetStaticMeshComponent))
  (bind _launchstrength (Variables|Default|GetLaunchStrength))
  (bind _returnvalue (Transformation|GetWorldLocation _staticmeshcomponent))
  (bind _capsulecomponent (Variables|/Script/Engine.Character|GetCapsuleComponent _player))
  (bind _returnvalue_2 (Transformation|GetWorldLocation _capsulecomponent))
  (bind _returnvalue_3 (- _returnvalue_2 _returnvalue))
  (bind _returnvalue_4 (Math|Vector|Normalize _returnvalue_3))
  (bind _returnvalue_5 (* _returnvalue_4 _launchstrength))
  ;[1 1 1] Character hit
  (Class|GP2Team10ProjectHealthComponent|DecreaseHealth (Variables|/Game/GameProject2/Core/Characters/BP_PlayerPawn.BP_PlayerPawn_C|GetBP_HealthComponent _player_2) 1)
  (Character|LaunchCharacter _player_2 (Math|Vector|MakeVector (.x _returnvalue_5) (.y _returnvalue_5) (+ (.z _returnvalue_5) (Variables|Default|GetHeightImpulse))) false false))

(event Custom|LookAtBoss
  (bind _returnvalue (Game|GetPlayerController 0))
  ;[1 1 1] CustomTick
  (Pawn|SetControlRotation _returnvalue (Math|Rotator|Lerp(Rotator) (Pawn|GetControlRotation _returnvalue :!class /Script/Engine.Controller) (Math|Rotator|FindLookatRotation (Transformation|GetWorldLocation (Variables|/Script/GP2Team10Project.GP2Team10ProjectPlayerCharacter|GetCameraBoom (Variables|Default|GetPlayer))) (Transformation|GetWorldLocation (Variables|Debug|GetStaticMeshComponent))) 0.01 true)))

(event EventBeginPlay
  (bind _asbp_player_pawn (Utilities|Casting|CastToBP_PlayerPawn (Pawn|GetControlledPawn (Game|GetPlayerController 0))))
  (Variables|Default|SetPlayer _asbp_player_pawn)
  (EventDispatchers|BindEventtoOnHealthZero (Variables|/Game/GameProject2/Core/Characters/BP_PlayerPawn.BP_PlayerPawn_C|GetBP_HealthComponent (Variables|Default|GetPlayer)) (delegate Custom|Death))
  (Variables|Default|SetHealth (Variables|Default|GetMaxHealth)))

(event EventTick
  (params (DeltaSeconds :type Float%20%28single-precision%29))
  (Utilities|FlowControl|Sequence
    (:then_0
      (if (Variables|Default|GetBossActive)
        (if (Variables|Default|GetFiringLaser)
          (bind _output_get (Variables|Default|SetLookAtRotation (Math|Rotator|FindLookatRotation (Transformation|GetWorldLocation (Variables|Default|GetLazerExit)) (Transformation|GetWorldLocation (Variables|/Script/Engine.Actor|GetRootComponent (Variables|Default|GetPlayer))))))
          (Transformation|SetWorldRotation (Variables|/Game/GameProject2/Core/Characters/Boss/BP_LaserIndicator.BP_LaserIndicator_C|GetDefaultSceneRoot (Variables|Default|GetLaserIndicator)) _output_get false false))
        (if (Variables|Default|GetIsAttacking)
          _
          (else
            (Transformation|SetWorldRotation (Variables|Debug|GetStaticMeshComponent) (Math|Rotator|Lerp(Rotator) (Transformation|GetWorldRotation (Variables|Debug|GetStaticMeshComponent)) (Math|Rotator|MakeRotator 0.0 0.0 (+ (.yaw (Math|Rotator|FindLookatRotation (Transformation|GetWorldLocation (Variables|Debug|GetStaticMeshComponent)) (Transformation|GetWorldLocation (Variables|/Script/Engine.Character|GetCapsuleComponent (Variables|Default|GetPlayer))))) -9e+01)) 0.1 true) false false)))
        (bind _outhit (Collision|LineTraceForObjects (Transformation|GetWorldLocation (Variables|Debug|GetStaticMeshComponent)) (Transformation|GetWorldLocation (Variables|/Script/Engine.Character|GetCapsuleComponent (Variables|Default|GetPlayer))) (Utilities|Array|MakeArray "ObjectTypeQuery3") true 0 "None"))
        (if (> (.distance _outhit) 2.4e+03)
          (Variables|Default|SetRangeInt 2)
          (elif (Math|Float|InRange(Float) (.distance _outhit) 1.6e+03 2.4e+03)
            (Variables|Default|SetRangeInt 1)
            (else
              (Variables|Default|SetRangeInt 0))))))))

(fn ConstructionScript)