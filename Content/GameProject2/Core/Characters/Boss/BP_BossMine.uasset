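; BP_BossMine is a homing mine in the boss fight that can hurt either the player or BP_Boss.
; When the player enters its overlap sphere, it plays a noise and is pushed toward them by a force each tick.
; Hitting the player launches them away and costs health; hitting the boss's crystal hitbox damages the boss.
; Either character's contact explodes and destroys it; checkpoint-steering logic is present but never runs.
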(event OnComponentBeginOverlap(Sphere1)
  (params (OverlappedComponent :type Primitive%20Component%20Object%20Reference) (OtherActor :type Actor%20Object%20Reference) (OtherComp :type Primitive%20Component%20Object%20Reference) (OtherBodyIndex :type Integer) (bFromSweep :type Boolean) (SweepResult :type Hit%20Result%20Structure%20%28by%20ref%29))
  ;[1 1 1] Homing function
  (if (== OtherActor (Variables|Default|GetPlayer))
    (Variables|Default|SetMovingToPlayer true)
    (Class|FMODBlueprintStatics|PlayEventAttached "/Game/FMOD/Events/Enemies/Mine/Mine_Noise.Mine_Noise" (Variables|Default|GetSphere) "None" "0, 0, 0" "KeepRelativeOffset")))

(event OnComponentHit(Sphere)
  (params (HitComponent :type Primitive%20Component%20Object%20Reference) (OtherActor :type Actor%20Object%20Reference) (OtherComp :type Primitive%20Component%20Object%20Reference) (NormalImpulse :type Vector :default "0, 0, 0") (Hit :type Hit%20Result%20Structure%20%28by%20ref%29))
  ;[1 1 1] Explosion
  (if (== OtherActor (Variables|Default|GetBoss))
    (if (== OtherComp (Variables|/Game/GameProject2/Core/Characters/Boss/BP_Boss.BP_Boss_C|GetCrystalHitbox (Variables|Default|GetBoss)))
      (Utilities|FlowControl|DoOnce false
        (:Completed
          (Default|BossTakeDmg (Variables|Default|GetBoss)))))
    (Niagara|SpawnSystematLocation "/Game/GameProject2/Effects/Systems/PS_MineExplosion.PS_MineExplosion" (Transformation|GetWorldLocation (Variables|Default|GetSphere)))
    (Actor|DestroyActor)
    (Class|FMODBlueprintStatics|PlayEventatLocation "/Game/FMOD/Events/Enemies/Mine/Mine_Explode.Mine_Explode" (Transformation|GetActorTransform))
    (elif (== OtherActor (Variables|Default|GetPlayer))
      (Character|LaunchCharacter (Variables|Default|GetPlayer) (* (Math|Vector|Normalize (- (Transformation|GetWorldLocation (Variables|/Script/Engine.Character|GetCapsuleComponent (Variables|Default|GetPlayer))) (Transformation|GetWorldLocation (Variables|Default|GetSphere)))) (Variables|Default|GetExplosionForce)) false false)
      (Niagara|SpawnSystematLocation "/Game/GameProject2/Effects/Systems/PS_MineExplosion.PS_MineExplosion" (Transformation|GetWorldLocation (Variables|Default|GetSphere)))
      (Class|GP2Team10ProjectHealthComponent|DecreaseHealth (Variables|/Game/GameProject2/Core/Characters/BP_PlayerPawn.BP_PlayerPawn_C|GetBP_HealthComponent (Variables|Default|GetPlayer)) 1)
      (Actor|DestroyActor))))

(event EventBeginPlay
  ;[1 1 1] Initial setup
  (bind _outactors (Actor|GetAllActorsOfClass "/Game/GameProject2/Core/Characters/Boss/BP_Boss.BP_Boss_C"))
  (Variables|Default|SetBoss (Utilities|Array|Get(acopy) _outactors))
  (bind _asbp_player_pawn (Utilities|Casting|CastToBP_PlayerPawn (Pawn|GetControlledPawn (Game|GetPlayerController 0))))
  (Variables|Default|SetPlayer _asbp_player_pawn))

(event EventTick
  (params (DeltaSeconds :type Float%20%28single-precision%29))
  ;[1 1 1] Tick
  (if (Variables|Default|GetMovingToPlayer)
    (Physics|AddForce (Variables|Default|GetSphere) (* (* (Math|Vector|Normalize (- (Transformation|GetWorldLocation (Variables|/Script/Engine.Character|GetCapsuleComponent (Variables|Default|GetPlayer))) (Transformation|GetWorldLocation (Variables|Default|GetSphere)))) (Variables|Default|GetForce)) (Utilities|Time|GetWorldDeltaSeconds)) "None" false)))

(fn ConstructionScript)