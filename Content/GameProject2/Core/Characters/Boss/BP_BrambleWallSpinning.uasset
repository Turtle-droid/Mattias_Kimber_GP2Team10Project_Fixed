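; A spinning bramble wall boss hazard that sweeps along negative world X, damaging and knocking back the player.
; BeginPlay sets a target 5000 units down that axis and attaches the Boss_Wave audio event to the cylinder.
; Tick spins the cylinder per frame, moves the root by Speed scaled by delta time, then stops audio and destroys itself near the target.
; Hitbox overlap removes health and launches the player away from the root.
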(event OnComponentBeginOverlap(Hitbox)
  (params (OverlappedComponent :type Primitive%20Component%20Object%20Reference) (OtherActor :type Actor%20Object%20Reference) (OtherComp :type Primitive%20Component%20Object%20Reference) (OtherBodyIndex :type Integer) (bFromSweep :type Boolean) (SweepResult :type Hit%20Result%20Structure%20%28by%20ref%29))
  (bind _asbp_player_pawn (Utilities|Casting|CastToBP_PlayerPawn OtherActor))
  (Utilities|FlowControl|DoOnce false :!label _label
    (:Completed
      (Class|GP2Team10ProjectHealthComponent|DecreaseHealth (Variables|/Game/GameProject2/Core/Characters/BP_PlayerPawn.BP_PlayerPawn_C|GetBP_HealthComponent _asbp_player_pawn) 1)
      (Character|LaunchCharacter _asbp_player_pawn (* (Math|Vector|Normalize (- (Transformation|GetWorldLocation (Variables|/Script/Engine.Character|GetCapsuleComponent _asbp_player_pawn)) (Transformation|GetWorldLocation (Variables|Default|GetDefaultSceneRoot)))) 2.5e+03) false false)
      (goto _label Reset))))

(event EventTick
  (params (DeltaSeconds :type Float%20%28single-precision%29))
  (Utilities|FlowControl|Sequence
    (:then_0
      (Transformation|AddLocalRotation (Variables|Default|GetCylinder) (Math|Rotator|MakeRotator 0.0 0.0 5.0) false false))
    (:then_3
      (Transformation|AddWorldOffset (Variables|Default|GetDefaultSceneRoot) (Math|Vector|MakeVector (* (* (Variables|Default|GetSpeed) -1.0) (Utilities|Time|GetWorldDeltaSeconds)) 0.0 0.0) false false)
      (if (Math|Vector|Equal(Vector) (Transformation|GetWorldLocation (Variables|Default|GetDefaultSceneRoot)) (Variables|Default|GetTarget) 1e+01)
        (Class|FMODAudioComponent|Stop (stale EventBeginPlay _returnvalue_2))
        (Actor|DestroyActor)))))

(event EventBeginPlay
  (bind _defaultsceneroot (Variables|Default|GetDefaultSceneRoot))
  (bind _returnvalue (Transformation|GetWorldLocation _defaultsceneroot))
  (Variables|Default|SetTarget (Math|Vector|MakeVector (- (.x _returnvalue) 5e+03) (.y _returnvalue) (.z _returnvalue)))
  (bind _returnvalue_2 (Class|FMODBlueprintStatics|PlayEventAttached "/Game/FMOD/Events/Enemies/Boss/Boss_Attacks/Boss_Wave.Boss_Wave" (Variables|Default|GetCylinder) "None" "0, 0, 0" "KeepRelativeOffset")))

(fn ConstructionScript)