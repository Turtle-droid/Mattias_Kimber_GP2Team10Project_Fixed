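; BP_Gamemode is a game mode that handles the loading screen at level start and the victory screen on a win.
; On BeginPlay it shows W_Loadingscreen and disables the player pawn's input for a fixed delay, then restores input and calls the HUD toggle.
; PlayerWin shows W_VictoryScreen with keyboard focus on its main menu exit button; the UI-only input and mouse cursor nodes are disconnected.
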(event Custom|PlayerWin
  (bind _returnvalue (UserInterface|CreateWidget "/Game/GameProject2/Core/MenuUI/W_VictoryScreen.W_VictoryScreen_C" (Game|GetPlayerController 0)))
  (UserInterface|Viewport|AddtoViewport _returnvalue 0)
  (Widget|SetKeyboardFocus (Variables|/Game/GameProject2/Core/MenuUI/W_VictoryScreen.W_VictoryScreen_C|GetExitToMainMenu _returnvalue)))

(event EventBeginPlay
  (bind _returnvalue (Game|GetPlayerController 0))
  (bind _returnvalue_2 (Game|GetPlayerController 0))
  (bind _returnvalue_3 (UserInterface|CreateWidget "/Game/GameProject2/Core/MenuUI/W_Loadingscreen.W_Loadingscreen_C" (Game|GetPlayerController 0)))
  (bind _output_get (Variables|Default|SetLoadingScren _returnvalue_3))
  (UserInterface|Viewport|AddtoViewport _output_get 0)
  (Input|DisableInput (Pawn|GetControlledPawn _returnvalue_2) _returnvalue_2)
  (Utilities|FlowControl|Delay 3.5)
  (Widget|RemovefromParent (Variables|Default|GetLoadingScren))
  (Input|EnableInput (Pawn|GetControlledPawn _returnvalue) _returnvalue)
  (Default|CallToggleHUD))

(fn ConstructionScript)