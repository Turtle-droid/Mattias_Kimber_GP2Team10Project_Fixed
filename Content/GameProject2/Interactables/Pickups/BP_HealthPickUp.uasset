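; BP_HealthPickUp is a pickup that restores one health point to the player pawn on overlap.
; A Do Once, reset when the pawn leaves, notifies the pawn, spawns a Niagara effect and plays a 2D pickup sound.
; Health rises through the pawn's health component only when below maximum, but the pickup destroys itself either way, so it is consumed at full health.
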(event Collision|EventActorBeginOverlap
  (params (OtherActor :type Actor%20Object%20Reference))
  (bind _asbp_player_pawn (Utilities|Casting|CastToBP_PlayerPawn OtherActor))
  (Utilities|FlowControl|DoOnce false
    (:Completed
      (Default|EventPickupTriggered _asbp_player_pawn)
      (Niagara|SpawnSystematLocation "/Game/GameProject2/Effects/Systems/PS_Checkpoint.PS_Checkpoint" (Transformation|GetWorldLocation (Variables|Default|GetNiagara)))
      (if (== (Class|GP2Team10ProjectHealthComponent|GetCurrentHealth (Variables|/Game/GameProject2/Core/Characters/BP_PlayerPawn.BP_PlayerPawn_C|GetBP_HealthComponent _asbp_player_pawn)) (Class|GP2Team10ProjectHealthComponent|GetMaxHealth (Variables|/Game/GameProject2/Core/Characters/BP_PlayerPawn.BP_PlayerPawn_C|GetBP_HealthComponent _asbp_player_pawn)))
        (Actor|DestroyActor)
        (else
          (Class|GP2Team10ProjectHealthComponent|IncreaseHealth (Variables|/Game/GameProject2/Core/Characters/BP_PlayerPawn.BP_PlayerPawn_C|GetBP_HealthComponent _asbp_player_pawn) 1)
          (Actor|DestroyActor)))
      (Class|FMODBlueprintStatics|PlayEvent2D "/Game/FMOD/Events/Interactables/Health_Pickup.Health_Pickup"))))

(event Collision|EventActorEndOverlap
  (params (OtherActor :type Actor%20Object%20Reference))
  (Utilities|Casting|CastToBP_PlayerPawn OtherActor)
  (Utilities|FlowControl|DoOnce false) ; enters at Reset
)

(fn ConstructionScript)