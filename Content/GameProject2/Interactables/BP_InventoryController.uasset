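; BP_InventoryController opens and closes the inventory screen in response to the OpenInventory input action.
; It creates the WB_Inventory widget on first open, keeps a reference to it, then toggles it by adding it to or removing it from the viewport.
; A ReloadInventory event tells an existing widget to reload its items through LoadInventoryItems.
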(event EventReloadInventory
  (bind _inventorywidget (Variables|Default|GetInventoryWidget))
  (Utilities|IsValid _inventorywidget
    (:Is%20Valid
      (Default|LoadInventoryItems (.AsWB%20Inventory (Utilities|Casting|CastToWB_Inventory _inventorywidget))))))

(event Input|ActionEvents|InputActionOpenInventory
  (params (Key :type Key%20Structure))
  (:Pressed
    (if (Widget|IsVisible (Variables|Default|GetInventoryWidget))
      (Widget|RemovefromParent (Variables|Default|GetInventoryWidget))
      (else
        (Utilities|IsValid (Variables|Default|GetInventoryWidget)
          (:Is%20Valid
            _)
          (:Is%20Not%20Valid
            (bind _returnvalue (UserInterface|CreateWidget "/Game/GameProject2/Interactables/UI/WB_Inventory.WB_Inventory_C"))
            (Variables|Default|SetInventoryWidget _returnvalue)))
        (UserInterface|Viewport|AddtoViewport (Variables|Default|GetInventoryWidget) 0)))))

(fn ConstructionScript)