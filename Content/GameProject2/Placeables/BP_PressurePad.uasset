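; BP_PressurePad is a placeable pressure pad that animates its mesh when activated or deactivated.
; BeginPlay stores the mesh's relative location and a target 10 units higher on Z, since it subtracts a negative offset.
; The activation event plays the FloatTrack timeline to lerp the mesh toward that target, and deactivation reverses it.
; The graph contains no trigger detection, only the responses to these two events.
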(event EventBeginPlay
  (bind _output_get (Variables|Default|SetMeshLocation (Variables|/Script/Engine.SceneComponent|GetRelativeLocation (Variables|Default|GetPressurePadMesh))))
  (Variables|Default|SetMeshTargetLocation (- _output_get (Math|Vector|MakeVector 0.0 0.0 -1e+01))))

(event EventOnPressurePadActivated
  (bind _floattrackk (Timeline|FloatTrack Play)
    (:Update
      (Transformation|SetRelativeLocation (Variables|Default|GetPressurePadMesh) (Math|Vector|Lerp(Vector) (Variables|Default|GetMeshLocation) (Variables|Default|GetMeshTargetLocation) _floattrackk) false false))))

(event EventOnPressurePadDeactivated
  (bind _floattrackk (Timeline|FloatTrack Reverse)
    (:Update
      (Transformation|SetRelativeLocation (Variables|Default|GetPressurePadMesh) (Math|Vector|Lerp(Vector) (Variables|Default|GetMeshLocation) (Variables|Default|GetMeshTargetLocation) _floattrackk) false false))))

(fn ConstructionScript)