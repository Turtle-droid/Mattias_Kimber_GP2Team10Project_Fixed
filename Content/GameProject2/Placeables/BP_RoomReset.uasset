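; Pressure-pad placeable that resets a room by returning a designated list of actors to their starting transforms.
; BeginPlay caches the pad mesh position and each listed actor's location and rotation.
; Activation marks every BP_RopePoints in the level, has the player pawn remove marked things, then zeroes the actors' linear velocity and restores their transforms.
; A timeline slides the pad mesh on activation and reverses on deactivation.
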(event EventBeginPlay
  (bind _output_get (Variables|Default|SetMeshLocation (Variables|/Script/Engine.SceneComponent|GetRelativeLocation (Variables|Default|GetPressurePadMesh))))
  (Variables|Default|SetMeshTargetLocation (- _output_get (Math|Vector|MakeVector 0.0 0.0 -1e+01)))
  (for _array_element (Variables|Default|GetActorsToReset)
    (Utilities|Array|Add (Variables|Default|GetActorLocations) (Transformation|GetActorLocation _array_element))
    (Utilities|Array|Add (Variables|Default|GetActorRotations) (Transformation|GetActorRotation _array_element))))

(event EventOnPressurePadActivated
  (bind _outactors (Actor|GetAllActorsOfClass "/Game/GameProject2/Core/Characters/BP_RopePoints.BP_RopePoints_C"))
  (for _array_element _outactors
    (Variables|/Game/GameProject2/Core/Characters/BP_RopePoints.BP_RopePoints_C|SetMarked _array_element true))
  (bind _asbp_player_pawn (Utilities|Casting|CastToBP_PlayerPawn (Pawn|GetControlledPawn (Game|GetPlayerController 0)))
    (:then
      (Default|RemoveMarkedThings _asbp_player_pawn))
    (:CastFailed
      _))
  (Utilities|FlowControl|Sequence
    (:then_0
      (for (_array_element_2 _array_index) (Variables|Default|GetActorLocations)
        (Physics|SetPhysicsLinearVelocity (Actor|GetComponentbyClass (Utilities|Array|Get(acopy) (Variables|Default|GetActorsToReset) _array_index) "/Script/Engine.StaticMeshComponent") "0, 0, 0" false "None")
        (Transformation|SetActorLocationAndRotation (Utilities|Array|Get(acopy) (Variables|Default|GetActorsToReset) _array_index) _array_element_2 (Utilities|Array|Get(acopy) (Variables|Default|GetActorRotations) _array_index))))
    (:then_1
      (bind _floattrackk (Timeline|FloatTrack Play)
        (:Update
          (Transformation|SetRelativeLocation (Variables|Default|GetPressurePadMesh) (Math|Vector|Lerp(Vector) (Variables|Default|GetMeshLocation) (Variables|Default|GetMeshTargetLocation) _floattrackk) false false))))))

(event EventOnPressurePadDeactivated
  (bind _floattrackk (Timeline|FloatTrack Reverse)
    (:Update
      (Transformation|SetRelativeLocation (Variables|Default|GetPressurePadMesh) (Math|Vector|Lerp(Vector) (Variables|Default|GetMeshLocation) (Variables|Default|GetMeshTargetLocation) _floattrackk) false false))))

(fn ConstructionScript)