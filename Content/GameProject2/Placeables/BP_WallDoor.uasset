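; BP_WallDoor is a placeable door that swings open when a pressure pad activates and swings back when it deactivates.
; A timeline plays forward or in reverse to yaw the root from its starting rotation, with a ChangeDirection flag choosing the swing direction.
; Each state change starts an attached Door_Opening sound event on the cube, which stops when the timeline finishes.
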(event EventBeginPlay
  (Variables|Default|SetInitalRotation (Transformation|GetWorldRotation (Variables|Default|GetDefaultSceneRoot)))
  (if (Variables|Default|GetChangeDirection)
    (Variables|Default|SetDirectionalChanger 1.0)
    (else
      (Variables|Default|SetDirectionalChanger -1.0))))

(event EventOnPressurePadActivated
  (Utilities|FlowControl|Sequence
    (:then_0
      (bind _openrotation (Timeline|OpenLine Stop)
        (:Update
          (Transformation|SetRelativeRotation (Variables|Default|GetDefaultSceneRoot) (Math|Rotator|MakeRotator 0.0 0.0 (+ (.yaw (Variables|Default|GetInitalRotation)) (* _openrotation (Variables|Default|GetDirectionalChanger)))) false false))
        (:Finished
          (bind _returnvalue (Class|FMODAudioComponent|IsPlaying (stale _returnvalue_2)))
          (if _returnvalue
            (Class|FMODAudioComponent|Stop (stale _returnvalue_2))))))
    (:then_1
      (Timeline|OpenLine Play))
    (:then_2
      (bind _returnvalue_2 (Class|FMODBlueprintStatics|PlayEventAttached "/Game/FMOD/Events/Enviroment/Door_Opening.Door_Opening" (Variables|Default|GetCube) "None" "0, 0, 0" "KeepRelativeOffset")))))

(event EventOnPressurePadDeactivated
  (Utilities|FlowControl|Sequence
    (:then_0
      (bind _openrotation (Timeline|OpenLine Stop)
        (:Update
          (Transformation|SetRelativeRotation (Variables|Default|GetDefaultSceneRoot) (Math|Rotator|MakeRotator 0.0 0.0 (+ (.yaw (Variables|Default|GetInitalRotation)) (* _openrotation (Variables|Default|GetDirectionalChanger)))) false false))
        (:Finished
          (bind _returnvalue (Class|FMODAudioComponent|IsPlaying (stale _returnvalue_2)))
          (if _returnvalue
            (Class|FMODAudioComponent|Stop (stale _returnvalue_2))))))
    (:then_1
      (Timeline|OpenLine Reverse))
    (:then_2
      (bind _returnvalue_2 (Class|FMODBlueprintStatics|PlayEventAttached "/Game/FMOD/Events/Enviroment/Door_Opening.Door_Opening" (Variables|Default|GetCube) "None" "0, 0, 0" "KeepRelativeOffset")))))

(fn ConstructionScript)