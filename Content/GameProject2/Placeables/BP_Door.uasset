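; Placeable door that swings open and closed around its yaw axis in response to pressure pad activated and deactivated events.
; On BeginPlay it stores the root's world rotation and turns the ChangeDirection flag into a swing sign.
; The OpenLine timeline plays on activation and reverses on deactivation, adding its signed rotation curve to the stored yaw and applying it as relative rotation.
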(event EventBeginPlay
  (Variables|Default|SetInitalRotation (Transformation|GetWorldRotation (Variables|Default|GetDefaultSceneRoot)))
  (if (Variables|Default|GetChangeDirection)
    (Variables|Default|SetDirectionalChanger 1.0)
    (else
      (Variables|Default|SetDirectionalChanger -1.0))))

(event EventOnPressurePadActivated
  (Utilities|FlowControl|Sequence
    (:then_0
      (bind _openrotation (Timeline|OpenLine Stop)
        (:Update
          (Transformation|SetRelativeRotation (Variables|Default|GetDefaultSceneRoot) (Math|Rotator|MakeRotator 0.0 0.0 (+ (.yaw (Variables|Default|GetInitalRotation)) (* _openrotation (Variables|Default|GetDirectionalChanger)))) false false))))
    (:then_1
      (Timeline|OpenLine Play))))

(event EventOnPressurePadDeactivated
  (Utilities|FlowControl|Sequence
    (:then_0
      (bind _openrotation (Timeline|OpenLine Stop)
        (:Update
          (Transformation|SetRelativeRotation (Variables|Default|GetDefaultSceneRoot) (Math|Rotator|MakeRotator 0.0 0.0 (+ (.yaw (Variables|Default|GetInitalRotation)) (* _openrotation (Variables|Default|GetDirectionalChanger)))) false false))))
    (:then_1
      (Timeline|OpenLine Reverse))))

(fn ConstructionScript)