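; BP_BreakableBossDoor is a placeable door that breaks when a boss mine hits it.
; Its HitBox hit event casts the other actor to BP_BossMine and uses a DoOnce so the break runs a single time.
; On that hit it destroys the mine, spawns explosion and damage effects, plays the crystal-breaking sound event, then destroys itself.
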(event OnComponentHit(HitBox)
  (params (HitComponent :type Primitive%20Component%20Object%20Reference) (OtherActor :type Actor%20Object%20Reference) (OtherComp :type Primitive%20Component%20Object%20Reference) (NormalImpulse :type Vector :default "0, 0, 0") (Hit :type Hit%20Result%20Structure%20%28by%20ref%29))
  (Variables|Default|SetOtherActor OtherActor)
  (bind _otheractor (Variables|Default|GetOtherActor)
    (:then
      (bind _asbp_boss_mine (Utilities|Casting|CastToBP_BossMine _otheractor))
      (Utilities|FlowControl|DoOnce false
        (:Completed
          (Actor|DestroyActor _asbp_boss_mine)
          (Niagara|SpawnSystematLocation "/Game/GameProject2/Effects/Systems/PS_MineExplosion.PS_MineExplosion" (.location Hit))
          (Class|FMODBlueprintStatics|PlayEventatLocation "/Game/FMOD/Events/Enviroment/Crystal_Breaking.Crystal_Breaking" (Transformation|GetActorTransform))
          (Niagara|SpawnSystematLocation "/Game/GameProject2/Effects/Systems/PS_Boss_Damage_FX.PS_Boss_Damage_FX" (Transformation|GetWorldLocation (Variables|Default|GetHitBox)))
          (Actor|DestroyActor))))
    (:else)))

(fn ConstructionScript)