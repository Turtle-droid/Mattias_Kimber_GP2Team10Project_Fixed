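; BP_SlideDoor is a placeable door that slides vertically in response to pressure pad activation and deactivation events.
; BeginPlay caches the root's world location and sets the slide sign from ChangeDirection, upward when true and downward otherwise.
; The OpenLine timeline plays on activation and reverses on deactivation, offsetting the root's Z from that start by its track value, which is named OpenRotation despite driving translation.
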(event EventBeginPlay
  (Variables|Default|SetInitialLocation (Transformation|GetWorldLocation (Variables|Default|GetDefaultSceneRoot)))
  (if (Variables|Default|GetChangeDirection)
    (Variables|Default|SetDirectionalChanger 1.0)
    (else
      (Variables|Default|SetDirectionalChanger -1.0))))

(event EventOnPressurePadActivated
  (bind _initiallocation (Variables|Default|GetInitialLocation))
  (Utilities|FlowControl|Sequence
    (:then_0
      (bind _openrotation (Timeline|OpenLine Stop)
        (:Update
          (Transformation|SetWorldLocation (Variables|Default|GetDefaultSceneRoot) (Math|Vector|MakeVector (.x _initiallocation) (.y _initiallocation) (+ (.z _initiallocation) (* _openrotation (Variables|Default|GetDirectionalChanger)))) false false))))
    (:then_1
      (Timeline|OpenLine Play))))

(event EventOnPressurePadDeactivated
  (bind _initiallocation (Variables|Default|GetInitialLocation))
  (Utilities|FlowControl|Sequence
    (:then_0
      (bind _openrotation (Timeline|OpenLine Stop)
        (:Update
          (Transformation|SetWorldLocation (Variables|Default|GetDefaultSceneRoot) (Math|Vector|MakeVector (.x _initiallocation) (.y _initiallocation) (+ (.z _initiallocation) (* _openrotation (Variables|Default|GetDirectionalChanger)))) false false))))
    (:then_1
      (Timeline|OpenLine Reverse))))

(fn ConstructionScript)