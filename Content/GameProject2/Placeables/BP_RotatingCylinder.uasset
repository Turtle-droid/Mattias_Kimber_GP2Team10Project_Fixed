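; A placeable physics obstacle: a spinning cylinder with hit components that knock the player away.
; Each tick it adds frame-scaled torque as an acceleration change on all three axes while angular speed stays under a fixed cap.
; When the cube or one of three static meshes hits the player pawn cached at BeginPlay, it launches the player outward from that component.
; The cylinder's own hit event does nothing.
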(event OnComponentHit(Cylinder)
  (params (HitComponent :type Primitive%20Component%20Object%20Reference) (OtherActor :type Actor%20Object%20Reference) (OtherComp :type Primitive%20Component%20Object%20Reference) (NormalImpulse :type Vector :default "0, 0, 0") (Hit :type Hit%20Result%20Structure%20%28by%20ref%29)))

(event OnComponentHit(Cube)
  (params (HitComponent :type Primitive%20Component%20Object%20Reference) (OtherActor :type Actor%20Object%20Reference) (OtherComp :type Primitive%20Component%20Object%20Reference) (NormalImpulse :type Vector :default "0, 0, 0") (Hit :type Hit%20Result%20Structure%20%28by%20ref%29))
  (if (== OtherActor (Variables|Default|GetPlayer))
    (Character|LaunchCharacter (Variables|Default|GetPlayer) (* (Math|Vector|Normalize (- (Transformation|GetWorldLocation (Variables|/Script/Engine.Character|GetCapsuleComponent (Variables|Default|GetPlayer))) (Transformation|GetWorldLocation (Variables|Default|GetCube)))) (Variables|Default|GetLaunchForce)) false false)))

(event OnComponentHit(StaticMesh)
  (params (HitComponent :type Primitive%20Component%20Object%20Reference) (OtherActor :type Actor%20Object%20Reference) (OtherComp :type Primitive%20Component%20Object%20Reference) (NormalImpulse :type Vector :default "0, 0, 0") (Hit :type Hit%20Result%20Structure%20%28by%20ref%29))
  (if (== OtherActor (Variables|Default|GetPlayer))
    (Character|LaunchCharacter (Variables|Default|GetPlayer) (* (Math|Vector|Normalize (- (Transformation|GetWorldLocation (Variables|/Script/Engine.Character|GetCapsuleComponent (Variables|Default|GetPlayer))) (Transformation|GetWorldLocation (Variables|Default|GetStaticMesh)))) (Variables|Default|GetLaunchForce)) false false)))

(event OnComponentHit(StaticMesh2)
  (params (HitComponent :type Primitive%20Component%20Object%20Reference) (OtherActor :type Actor%20Object%20Reference) (OtherComp :type Primitive%20Component%20Object%20Reference) (NormalImpulse :type Vector :default "0, 0, 0") (Hit :type Hit%20Result%20Structure%20%28by%20ref%29))
  (if (== OtherActor (Variables|Default|GetPlayer))
    (Character|LaunchCharacter (Variables|Default|GetPlayer) (* (Math|Vector|Normalize (- (Transformation|GetWorldLocation (Variables|/Script/Engine.Character|GetCapsuleComponent (Variables|Default|GetPlayer))) (Transformation|GetWorldLocation (Variables|Default|GetStaticMesh2)))) (Variables|Default|GetLaunchForce)) false false)))

(event OnComponentHit(StaticMesh1)
  (params (HitComponent :type Primitive%20Component%20Object%20Reference) (OtherActor :type Actor%20Object%20Reference) (OtherComp :type Primitive%20Component%20Object%20Reference) (NormalImpulse :type Vector :default "0, 0, 0") (Hit :type Hit%20Result%20Structure%20%28by%20ref%29))
  (if (== OtherActor (Variables|Default|GetPlayer))
    (Character|LaunchCharacter (Variables|Default|GetPlayer) (* (Math|Vector|Normalize (- (Transformation|GetWorldLocation (Variables|/Script/Engine.Character|GetCapsuleComponent (Variables|Default|GetPlayer))) (Transformation|GetWorldLocation (Variables|Default|GetStaticMesh1)))) (Variables|Default|GetLaunchForce)) false false)))

(event EventTick
  (params (DeltaSeconds :type Float%20%28single-precision%29))
  (bind _returnvalue (Utilities|Time|GetWorldDeltaSeconds))
  (bind _rotationspeed (Variables|Default|GetRotationSpeed))
  (bind _returnvalue_2 (* _rotationspeed _returnvalue))
  (if (< (Math|Vector|VectorLength (Physics|GetPhysicsAngularVelocityinDegrees (Variables|Default|GetCylinder) "None")) 1e+02)
    (Class|PrimitiveComponent|AddTorqueinDegrees (Variables|Default|GetCylinder) (Math|Vector|MakeVector _returnvalue_2 _returnvalue_2 _returnvalue_2) "None" true)))

(event EventBeginPlay
  (bind _asbp_player_pawn (Utilities|Casting|CastToBP_PlayerPawn (Pawn|GetControlledPawn (Game|GetPlayerController 0))))
  (Variables|Default|SetPlayer _asbp_player_pawn))

(fn ConstructionScript)