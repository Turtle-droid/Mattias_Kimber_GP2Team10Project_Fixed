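; BP_BossElevator is a boss elevator platform that carries the player up when they enter its trigger box.
; On overlap, a timeline raises the mesh from its starting location while the player's jump is disabled, then restores jumping.
; CallDown lowers the raised platform with a second timeline.
; DoOnce gates block retriggering and reset once the descent finishes, readying another ride.
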(event OnComponentBeginOverlap(Box)
  (params (OverlappedComponent :type Primitive%20Component%20Object%20Reference) (OtherActor :type Actor%20Object%20Reference) (OtherComp :type Primitive%20Component%20Object%20Reference) (OtherBodyIndex :type Integer) (bFromSweep :type Boolean) (SweepResult :type Hit%20Result%20Structure%20%28by%20ref%29))
  (bind _cachedlocation (Variables|Default|GetCachedLocation))
  (bind _asbp_player_pawn (Utilities|Casting|CastToBP_PlayerPawn OtherActor))
  (Variables|Default|SetPlayer _asbp_player_pawn)
  (Utilities|FlowControl|Sequence
    (:then_0
      (Utilities|FlowControl|DoOnce false
        (:Completed
          (Variables|/Script/Engine.Character|SetJumpMaxCount (Variables|Default|GetPlayer) 0))))
    (:then_1
      (Utilities|FlowControl|DoOnce false
        (:Completed
          (bind _goup (Timeline|GoUp PlayFromStart)
            (:Update
              (Transformation|SetWorldLocation (Variables|Debug|GetStaticMeshComponent) (Math|Vector|MakeVector (.x _cachedlocation) (.y _cachedlocation) (+ (.z _cachedlocation) _goup)) false false))
            (:Finished
              (Variables|/Script/Engine.Character|SetJumpMaxCount (Variables|Default|GetPlayer) 1)
              (Variables|Default|SetElevatorUp true))))))))

(event Custom|CallDown
  (bind _cachedlocation (Variables|Default|GetCachedLocation))
  (bind _staticmeshcomponent (Variables|Debug|GetStaticMeshComponent))
  (bind _returnvalue (Transformation|GetWorldLocation _staticmeshcomponent))
  (if (Variables|Default|GetElevatorUp)
    (Utilities|FlowControl|DoOnce false :!label _label
      (:Completed
        (bind _output_get (Variables|Default|SetCachedZLocation (.z _returnvalue)))
        (bind _goup (Timeline|Timeline_0 PlayFromStart)
          (:Update
            (Transformation|SetWorldLocation (Variables|Debug|GetStaticMeshComponent) (Math|Vector|MakeVector (.x _returnvalue) (.y _returnvalue) (- _output_get _goup)) false false))
          (:Finished
            (Variables|Default|SetElevatorUp false)
            (Utilities|FlowControl|Sequence
              (:then_0
                (goto _label Reset))
              (:then_1
                (Utilities|FlowControl|DoOnce false) ; enters at Reset
              )
              (:then_2
                (Utilities|FlowControl|DoOnce false) ; enters at Reset
              ))))))))

(event EventBeginPlay
  (Variables|Default|SetCachedLocation (Transformation|GetWorldLocation (Variables|Debug|GetStaticMeshComponent))))

(fn ConstructionScript)