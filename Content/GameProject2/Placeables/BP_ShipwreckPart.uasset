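; BP_ShipwreckPart is a placeable checkpoint that plays an attached shipwreck tune from BeginPlay.
; The first BP_PlayerPawn overlap of its Box, gated by DoOnce, sets the pawn's TargetLocation to NextCheckpoint and moves its respawn point to the part's spawn scene.
; It then swaps Cube materials to an active crystal, spawns checkpoint and sparkle effects, and plays a music stinger.
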(event OnComponentBeginOverlap(Box)
  (params (OverlappedComponent :type Primitive%20Component%20Object%20Reference) (OtherActor :type Actor%20Object%20Reference) (OtherComp :type Primitive%20Component%20Object%20Reference) (OtherBodyIndex :type Integer) (bFromSweep :type Boolean) (SweepResult :type Hit%20Result%20Structure%20%28by%20ref%29))
  (bind _crystal (Variables|Default|GetCrystal))
  (bind _asbp_player_pawn (Utilities|Casting|CastToBP_PlayerPawn OtherActor))
  (Utilities|FlowControl|DoOnce false
    (:Completed
      (Variables|/Game/GameProject2/Core/Characters/BP_PlayerPawn.BP_PlayerPawn_C|SetTargetLocation _asbp_player_pawn (Variables|Default|GetNext%20Checkpoint))
      (Class|GP2Team10ProjectPlayerCharacter|ChangeCurrentRespawnPoint _asbp_player_pawn (Transformation|GetWorldLocation (Variables|Default|GetSpawningPointScene)) "0, 0, 0")
      (Rendering|Material|SetMaterial (Variables|Default|GetCube) 0 "/Game/GameProject2/Effects/FXAssets/MI_Active_Crystal.MI_Active_Crystal")
      (Rendering|Material|SetMaterial (Variables|Default|GetCube) 2 "/Game/GameProject2/Effects/FXAssets/MI_Active_Crystal.MI_Active_Crystal")
      (Niagara|SpawnSystematLocation "/Game/GameProject2/Effects/Systems/PS_Checkpoint.PS_Checkpoint" (Transformation|GetWorldLocation _crystal) (Transformation|GetWorldRotation _crystal))
      (Niagara|SpawnSystematLocation "/Game/GameProject2/Effects/Systems/PS_CheckpointSparkles.PS_CheckpointSparkles" (Transformation|GetWorldLocation (Variables|Default|GetScene)))
      (Class|FMODBlueprintStatics|PlayEvent2D "/Game/FMOD/Events/Enviroment/Music_Stinger.Music_Stinger"))))

(event EventBeginPlay
  (Class|FMODBlueprintStatics|PlayEventAttached "/Game/FMOD/Events/Music/Shipwreck_Tune.Shipwreck_Tune" (Variables|Default|GetCube) "None" "0, 0, 0" "KeepRelativeOffset"))

(fn ConstructionScript)